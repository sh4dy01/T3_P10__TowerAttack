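; Combo attack component that plays the next montage from a list on each attack, or a separate in-air montage when the owner is falling.
; Starting is gated on not being in use or mid-attack, and the owner's walk speed is zeroed during the montage.
; Blend out advances the wrapping combo index for ground attacks, then ends the attack and restores speed.
; Cancelling also resets the combo, while TryEndAttack does nothing.
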(event `self.ExecuteAttack`
  (bind _charactermovement (`Character.CharacterMovement` (`self.Owner`)))
  (set `self.InitialSpeed` (`MovementComponent.GetMaxSpeed` _charactermovement))
  (set `CharacterMovementComponent.MaxWalkSpeed` 0.0 _charactermovement)
  (set `self.IsInCombo` true)
  (if (`NavMovementComponent.IsFalling` _charactermovement)
    ;[0.5212 1 0.6338] Play 'in-air' anim montage if the player is falling
    (`|PlayMontage` (`Character.Mesh` (`self.Owner`)) (`self.InAirAttackMontage`)
      (:`OnBlendOut`
        (`self.EndAttack`)))
    (else
      ;[0.4646 1 0.5279] Play next animation in combo
      (`|PlayMontage` (`Character.Mesh` (`self.Owner`)) (`|GetArrayItem` (`self.AttackAnimMontages`) (`self.CurrentAnimMontage`))
        (:`OnBlendOut`
          (bind _result (`/Engine/EditorBlueprintResources/StandardMacros.IncrementInt` (`self.CurrentAnimMontage`))
            (:`  `
              (set `self.CurrentAnimMontage` (mod _result (`KismetArrayLibrary.Array_Length` (`self.AttackAnimMontages`))))
              (`self.EndAttack`))))))))

(fn `CancelAttack`
  (`parent.CancelAttack`)
  (set `self.CurrentAnimMontage` 0)
  (set `self.IsInCombo` false)
  (`self.RevertSpeedToDefault`)
  (return))

(fn `EndAttack`
  (`KismetSystemLibrary.PrintString` "End combo")
  (set `self.IsInCombo` false)
  (`self.RevertSpeedToDefault`)
  (`parent.EndAttack`))

(fn `RevertSpeedToDefault`
  (set `CharacterMovementComponent.MaxWalkSpeed` (`self.InitialSpeed`) (`Character.CharacterMovement` (`self.Owner`))))

(fn `TryEndAttack`)

(fn `TryStartAttack`
  (if (not (`self.IsInUse`))
    (if (not (`self.IsInCombo`))
      (`self.StartAttack`)
      (`self.ExecuteAttack`))))