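; Attack component that runs a montage-driven melee combo on its owner, or an in-air attack montage when the owner is falling.
; Re-triggering during the combo montage sets IsInCombo; montage notifies consume that flag to advance ComboIndex, otherwise they end the attack.
; OnNextCombo broadcasts each index, switching movement to Flying on index 3 and Walking otherwise.
; Ending resets the combo and stops its montage; cancelling restores walk speed.
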(event `self.ReceiveBeginPlay`
  (`parent.ReceiveBeginPlay`)
  (add `self.OnNextCombo` (`|CreateDelegate` :!event `OnNextCombo_Event`)))

(event `self.ExecuteAttack`
  (if (`NavMovementComponent.IsFalling` (`Character.CharacterMovement` (`self.Owner`)))
    (`|PlayMontage` (`Character.Mesh` (`self.Owner`)) (`self.InAirAttackMontage`)
      (:`OnBlendOut`
        (`self.EndAttack`)))
    (elif (`AnimInstance.Montage_IsPlaying` (`SkeletalMeshComponent.GetAnimInstance` (`Character.Mesh` (`self.Owner`))) "/Game/Game/Blueprints/Characters/Juan/Animations/AM_JuanCombo.AM_JuanCombo")
      (set `self.IsInCombo` true)
      (else
        ;[1 1 1] Next combo
        (bind _result (`/Engine/EditorBlueprintResources/StandardMacros.IncrementInt` (`self.ComboIndex`))
          (:`  `
            (`self.OnNextCombo` _result)
            (`|PlayMontage` (`Character.Mesh` (`self.Owner`)) (`self.ComboMontage`) 1.5
              (:`OnCompleted`
                (`self.EndAttack`))
              (:`OnNotifyBegin`
                (if (`self.IsInCombo`)
                  (set `self.IsInCombo` false)
                  (bind _result_2 (`/Engine/EditorBlueprintResources/StandardMacros.IncrementInt` (`self.ComboIndex`))
                    (:`  `
                      (`self.OnNextCombo` _result_2)))
                  (else
                    (`self.EndAttack`)))))))))))

(event `OnNextCombo_Event` :!signature `self.OnNextCombo`
  (params (`Combo Index` :type Integer))
  (bind _charactermovement (`Character.CharacterMovement` (`self.Owner`)))
  (`|ExecutionSequence`
    (:`then_0`
      (switch `int` `Combo Index`
        (:`Default`
          (`CharacterMovementComponent.SetMovementMode` _charactermovement "MOVE_Walking" 0))
        (:`3`
          (`KismetSystemLibrary.PrintString` "flying")
          (`CharacterMovementComponent.SetMovementMode` _charactermovement "MOVE_Flying" 0))))))

(fn `CancelAttack`
  (`parent.CancelAttack`)
  (set `self.IsInCombo` false)
  (`self.RevertSpeedToDefault`)
  (return))

(fn `EndAttack`
  (bind _returnvalue (`SkeletalMeshComponent.GetAnimInstance` (`Character.Mesh` (`self.Owner`))))
  (`KismetSystemLibrary.PrintString` "End combo")
  (set `self.IsInCombo` false)
  (bind _output_get (set `self.ComboIndex` 0))
  (`self.OnNextCombo` _output_get)
  (if (`AnimInstance.Montage_IsPlaying` _returnvalue (`self.ComboMontage`))
    (`AnimInstance.Montage_Stop` _returnvalue 0.2 (`self.ComboMontage`))
    (`parent.EndAttack`)
    (else
      (`parent.EndAttack`))))

(fn `RevertSpeedToDefault`
  (set `CharacterMovementComponent.MaxWalkSpeed` (`self.InitialSpeed`) (`Character.CharacterMovement` (`self.Owner`))))

(fn `TryEndAttack`)

(fn `TryStartAttack`
  (if (`self.IsInUse`)
    ;[1 1 1] If is in combo
    (`self.ExecuteAttack`)
    (else
      (`self.StartAttack`)
      (`self.ExecuteAttack`))))