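; Base attack component that adds a cooldown between uses of an attack.
; TryStartAttack runs start, execute and end in sequence, only when the attack is neither in use nor cooling down.
; The EndAttack override calls the parent, then starts the cooldown, which holds an IsInCooldown flag for CooldownDelay and prints a debug message.
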(event `StartCooldown`
  (`KismetSystemLibrary.PrintString` "Cooldown started")
  (set `self.IsInCooldown` true)
  (`KismetSystemLibrary.Delay` (`self.CooldownDelay`))
  (set `self.IsInCooldown` false))

(fn `EndAttack`
  (`parent.EndAttack`)
  (`self.StartCooldown`)
  (return))

(fn `TryStartAttack`
  (if (not (`self.IsInUse`))
    (if (not (`self.IsInCooldown`))
      (`self.StartAttack`)
      (`self.ExecuteAttack`)
      (`self.EndAttack`))))