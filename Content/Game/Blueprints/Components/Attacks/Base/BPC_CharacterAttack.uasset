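; Base actor component for character attacks, providing the start and end lifecycle around attack logic that child classes write by overriding ExecuteAttack.
; It caches its BP_CharacterBase owner on BeginPlay and prints a message if the cast fails.
; TryStartAttack ignores calls while IsInUse is set, otherwise it sets the flag, broadcasts the used events and runs ExecuteAttack.
; Release or cancel ends an active attack, clearing the flag and broadcasting OnEnded.
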(event `self.ReceiveBeginPlay`
  (bind _asbp_character_base (cast `/Game/Game/Blueprints/Characters/BP_CharacterBase` (`self.GetOwner`))
    (:`then`
      (set `self.Owner` _asbp_character_base))
    (:`CastFailed`
      (`KismetSystemLibrary.PrintString` "Owner isn't a playable character"))))

(event `ExecuteAttack`)

(fn `CancelAttack`
  (if (`self.IsInUse`)
    (`self.EndAttack`)
    (return)))

(fn `EndAttack`
  (set `self.IsInUse` false)
  (`self.OnEnded`)
  (return))

(fn `OnRelease`
  (if (`self.IsInUse`)
    (`self.EndAttack`)
    (return)))

(fn `StartAttack`
  (set `self.IsInUse` true)
  (`self.OnUsed`)
  (`self.OnAttackUsed` self)
  (return))

(fn `TryStartAttack`
  (if (not (`self.IsInUse`))
    (`self.StartAttack`)
    (`self.ExecuteAttack`)))