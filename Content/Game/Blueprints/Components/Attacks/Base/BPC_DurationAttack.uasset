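; BPC_DurationAttack is an attack component for attacks that run over time, capped by a maximum duration timer.
; StartAttack runs the parent start, then starts a one-shot timer.
; EndAttack, only while that timer is active, adds elapsed time times a multiplier onto the existing CooldownDelay, clears the timer and calls the parent end.
; CancelAttack clears the timer without changing cooldown, then calls the parent cancel.
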(fn `CancelAttack`
  (if (`KismetSystemLibrary.K2_IsTimerActiveHandle` (`self.TimerHandle`))
    (`KismetSystemLibrary.K2_ClearAndInvalidateTimerHandle` (`self.TimerHandle`)))
  (`parent.CancelAttack`))

(fn `EndAttack`
  (bind _returnvalue (`KismetSystemLibrary.K2_GetTimerElapsedTimeHandle` (`self.TimerHandle`)))
  (`KismetSystemLibrary.PrintString` "end")
  (if (`KismetSystemLibrary.K2_IsTimerActiveHandle` (`self.TimerHandle`))
    (bind _output_get (set `self.TimeElapsed` _returnvalue))
    (`KismetSystemLibrary.PrintString` (`KismetStringLibrary.Conv_DoubleToString` _output_get))
    (set `self.CooldownDelay` (+ (`self.CooldownDelay`) (* _returnvalue (`self.DurationCooldownMultiplier`))))
    (`KismetSystemLibrary.K2_ClearAndInvalidateTimerHandle` (`self.TimerHandle`))
    (`parent.EndAttack`)
    (return)
    (else
      (`KismetSystemLibrary.PrintString` "Non"))))

(fn `StartAttack`
  (`KismetSystemLibrary.PrintString` "Start")
  (`parent.StartAttack`)
  (bind _returnvalue (`KismetSystemLibrary.K2_SetTimerDelegate` (`|CreateDelegate` :!event `EndAttack`) (`self.AttackMaxDuration`)))
  (set `self.TimerHandle` _returnvalue)
  (`KismetSystemLibrary.PrintString` "set timer"))