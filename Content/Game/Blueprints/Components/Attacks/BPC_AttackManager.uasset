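; Attack manager component that registers a primary attack, secondary attack and two spells in a map keyed by attack type.
; It binds to each attack's used and ended events and keeps track of the current attack and attacking state.
; Starts require attacking to be enabled and no attack in progress, unless repeating a repeatable current attack.
; It also forwards input releases and can end or cancel the current attack.
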(fn `BindEventToAttack`
  (params (Attack :type "/Game/Game/Blueprints/Components/Attacks/Base/BPC_CharacterAttack Object Reference"))
  (add `/Game/Game/Blueprints/Components/Attacks/Base/BPC_CharacterAttack.OnEnded` Attack (`|CreateDelegate` :!event `SetNotInAttack`))
  (add `/Game/Game/Blueprints/Components/Attacks/Base/BPC_CharacterAttack.OnUsed` Attack (`|CreateDelegate` :!event `SetInAttack`))
  (add `/Game/Game/Blueprints/Components/Attacks/Base/BPC_CharacterAttack.OnEnded` Attack (`|CreateDelegate` :!event `ResetCurrentAttack`))
  (add `/Game/Game/Blueprints/Components/Attacks/Base/BPC_CharacterAttack.OnAttackUsed` Attack (`|CreateDelegate` :!event `SetCurrentAttack`))
  (return))

(fn `DisableAttackAbility`
  (set `self.CanAttack` false))

(fn `EnableAttackAbility`
  (set `self.CanAttack` true))

(fn `Initialize`
  (params (PrimaryAttack :type "/Game/Game/Blueprints/Components/Attacks/Base/BPC_CharacterAttack Object Reference") (SecondaryAttack :type "/Game/Game/Blueprints/Components/Attacks/Base/BPC_CharacterAttack Object Reference") (FirstSpell :type "/Game/Game/Blueprints/Components/Attacks/Base/BPC_CharacterAttack Object Reference") (SecondSpell :type "/Game/Game/Blueprints/Components/Attacks/Base/BPC_CharacterAttack Object Reference"))
  (`self.RegisterAttack` "NewEnumerator0" PrimaryAttack)
  (`self.RegisterAttack` "NewEnumerator1" SecondaryAttack)
  (`self.RegisterAttack` "NewEnumerator2" FirstSpell)
  (`self.RegisterAttack` "NewEnumerator3" SecondSpell)
  (return))

(fn `RegisterAttack`
  (params (Attacktype :type "/Game/Game/Blueprints/Structs/E_AttackType Enum" :default "NewEnumerator0") (Attack :type "/Game/Game/Blueprints/Components/Attacks/Base/BPC_CharacterAttack Object Reference"))
  (`/Engine/EditorBlueprintResources/StandardMacros.IsValid` Attack
    (:`Is Valid`
      (`BlueprintMapLibrary.Map_Add` (`self.AllAttacks`) Attacktype Attack)
      (`self.BindEventToAttack` Attack)
      (return))
    (:`Is Not Valid`
      (`KismetSystemLibrary.PrintString` (`KismetStringLibrary.Concat_StrStr` "Can't set attack of type " (`|GetEnumeratorNameAsString` Attacktype))))))

(fn `ResetCurrentAttack`
  (set `self.CurrentAttack` null)
  (return))

(fn `SetCurrentAttack`
  (params (LastUsedAttack :type "/Game/Game/Blueprints/Components/Attacks/Base/BPC_CharacterAttack Object Reference"))
  (set `self.CurrentAttack` LastUsedAttack)
  (return))

(fn `SetInAttack`
  (set `self.IsAttacking` true))

(fn `SetNotInAttack`
  (set `self.IsAttacking` false))

(fn `TryCancelCurrentAttack`
  (bind _currentattack (`self.CurrentAttack`))
  (`/Engine/EditorBlueprintResources/StandardMacros.IsValid` _currentattack
    (:`Is Valid`
      (if (`/Game/Game/Blueprints/Components/Attacks/Base/BPC_CharacterAttack.IsInUse` _currentattack)
        (`/Game/Game/Blueprints/Components/Attacks/Base/BPC_CharacterAttack.CancelAttack` _currentattack)
        (`self.ResetCurrentAttack`)
        (return)))))

(fn `TryEndCurrentAttack`
  (bind _currentattack (`self.CurrentAttack`))
  (`/Engine/EditorBlueprintResources/StandardMacros.IsValid` _currentattack
    (:`Is Valid`
      (if (`/Game/Game/Blueprints/Components/Attacks/Base/BPC_CharacterAttack.IsInUse` _currentattack)
        (`/Game/Game/Blueprints/Components/Attacks/Base/BPC_CharacterAttack.EndAttack` _currentattack)
        (`self.ResetCurrentAttack`)
        (return)))))

(fn `TryReleaseAttackOfType`
  (params (AttackType :type "/Game/Game/Blueprints/Structs/E_AttackType Enum" :default "NewEnumerator0"))
  (bind (_value _returnvalue) (`BlueprintMapLibrary.Map_Find` (`self.AllAttacks`) AttackType))
  (if _returnvalue
    (`/Game/Game/Blueprints/Components/Attacks/Base/BPC_CharacterAttack.OnRelease` _value)
    (return)))

(fn `TryStartAttackOfType`
  (params (AttackType :type "/Game/Game/Blueprints/Structs/E_AttackType Enum" :default "NewEnumerator0"))
  (bind (_value _returnvalue) (`BlueprintMapLibrary.Map_Find` (`self.AllAttacks`) AttackType))
  (if (`self.CanAttack`)
    (if _returnvalue
      (if (not (`self.IsAttacking`))
        (`/Game/Game/Blueprints/Components/Attacks/Base/BPC_CharacterAttack.TryStartAttack` _value :!label _label)
        (return)
        (elif (and (`/Game/Game/Blueprints/Components/Attacks/Base/BPC_CharacterAttack.IsRepettable` _value) (== _value (`self.CurrentAttack`)))
          (goto _label))))))