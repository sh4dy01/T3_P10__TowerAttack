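; BPC_ShieldSpell is Juan's shield spell attack component, which places a shield actor at a scanner's position.
; Starting the attack shows the ShieldScanner mesh as a preview; release hides it and, if the scanner is not overlapping, plays the defend montage and spawns the shield slightly raised.
; Only one shield persists: a new one destroys the previous via NukeSelf, and EndAttack is called only in that replacement branch.
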(event `Init`
  (params (ShieldScanner :type "/Game/Game/Blueprints/Characters/Juan/BP_ShieldScanner Object Reference"))
  (set `self.Shield Scanner` ShieldScanner))

(event `PlayDefendAnimation`
  (bind _owner (`self.Owner`)
    (:`then`
      (`|PlayMontage` (`Character.Mesh` _owner) "/Game/Game/Blueprints/Characters/Juan/Animations/AM_JuanDefend.AM_JuanDefend" 2.0))
    (:`else`)))

(fn `EndAttack`
  (`parent.EndAttack`))

(fn `OnRelease`
  (bind _shield_scanner (`self.Shield Scanner`))
  (if (`self.IsInUse`)
    (`SceneComponent.SetVisibility` (`/Game/Game/Blueprints/Characters/Juan/BP_ShieldScanner.Mesh` (`self.Shield Scanner`)) false false)
    (if (not (`/Game/Game/Blueprints/Characters/Juan/BP_ShieldScanner.IsOverlapping` (`self.Shield Scanner`)))
      (`self.PlayDefendAnimation`)
      (bind _returnvalue (`|SpawnActorFromClass` (`self.ShieldClass`) (`KismetMathLibrary.MakeTransform` (+ (`Actor.K2_GetActorLocation` _shield_scanner) (0.0 0.0 100.0)) (`Actor.K2_GetActorRotation` _shield_scanner)) "AdjustIfPossibleButAlwaysSpawn" "MultiplyWithRoot" null null))
      (bind _previousshield (`self.PreviousShield`)
        (:`then`
          (`/Game/Game/Blueprints/Characters/Juan/BP_Shield.NukeSelf` _previousshield)
          (set `self.PreviousShield` _returnvalue)
          (`self.EndAttack`))
        (:`else`
          (set `self.PreviousShield` _returnvalue))))))

(fn `StartAttack`
  (`parent.StartAttack`)
  (`SceneComponent.SetVisibility` (`/Game/Game/Blueprints/Characters/Juan/BP_ShieldScanner.Mesh` (`self.Shield Scanner`)) true false))

(fn `TryStartAttack`
  (`parent.TryStartAttack`))