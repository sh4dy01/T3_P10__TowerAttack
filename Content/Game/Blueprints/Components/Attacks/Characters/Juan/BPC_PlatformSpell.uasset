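; Attack component for Juan's platform spell, which places a platform at the position and rotation of a scanner actor supplied through Init.
; Starting the attack shows the scanner's mesh; releasing while in use hides it and spawns the platform if the scanner is not overlapping.
; Only one platform persists: each successful cast nukes the previous one before ending the attack.
; An overlapping scanner cancels the attack, clearing the in-use flag and signalling that it ended.
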(event `Init`
  (params (PlatformScanner :type "/Game/Game/Blueprints/Characters/Juan/BP_PlatformScanner Object Reference"))
  (set `self.ScannerRef` PlatformScanner))

(fn `CancelAttack`
  (set `self.IsInUse` false)
  (`self.OnEnded`)
  (return))

(fn `OnRelease`
  (bind _scannerref (`self.ScannerRef`))
  ;[1 1 1] Checks to see if we can spawn a platform and makes the scanner invisible
  (if (`self.IsInUse`)
    (`SceneComponent.SetVisibility` (`/Game/Game/Blueprints/Characters/Juan/BP_Scanner.Mesh` (`self.ScannerRef`)) false false)
    (if (not (`/Game/Game/Blueprints/Characters/Juan/BP_Scanner.IsOverlapping` (`self.ScannerRef`)))
      ;[1 1 1] Spawn new platform and destroys the last one
      (bind _returnvalue (`|SpawnActorFromClass` (`self.PlatformClass`) (`KismetMathLibrary.MakeTransform` (`Actor.K2_GetActorLocation` _scannerref) (`Actor.K2_GetActorRotation` _scannerref)) "Undefined" "MultiplyWithRoot" null null))
      (bind _platformref (`self.PlatformRef`)
        (:`then`
          (`/Game/Game/Blueprints/Characters/Juan/BP_Platform.NukeSelf` _platformref)
          (set `self.PlatformRef` _returnvalue)
          (`self.EndAttack`))
        (:`else`
          (set `self.PlatformRef` _returnvalue)
          (`self.EndAttack`)))
      (else
        (`self.CancelAttack`)))))

(fn `StartAttack`
  (`parent.StartAttack`)
  (`SceneComponent.SetVisibility` (`/Game/Game/Blueprints/Characters/Juan/BP_Scanner.Mesh` (`self.ScannerRef`)) true false))