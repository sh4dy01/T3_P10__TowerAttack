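; Scotty's grab attack component, which picks up tagged grabbable items in view and throws them.
; Each tick a camera line trace highlights the grabbable item in range and resets the previous highlight.
; StartAttack grabs the highlighted item, or releases the held one with an impulse along the camera forward.
; A physics handle and socket passed through Init carry the item, with the target updated every tick.
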(event `self.ReceiveTick`
  (params (DeltaSeconds :type "Float (single-precision)"))
  (`parent.ReceiveTick` DeltaSeconds)
  (`self.CheckForGrabbableInSight`)
  ;[1 1 1] Grabbed Object Update
  (`/Engine/EditorBlueprintResources/StandardMacros.IsValid` (`self.GrabbedObject`)
    (:`Is Valid`
      (`PhysicsHandleComponent.SetTargetLocation` (`self.Grabber`) (`SceneComponent.K2_GetComponentLocation` (`self.Grab Socket`))))))

(event `Init`
  (params (`Physics Handle` :type "PhysicsHandleComponent Object Reference") (`Grab Socket` :type "ArrowComponent Object Reference"))
  (set `self.Grabber` `Physics Handle`)
  (set `self.Grab Socket` `Grab Socket`))

(fn `CheckForGrabbableInSight`
  (locals (bHit :type Boolean) (HitResult :type "HitResult Structure"))
  (bind _hightlightitem (`self.HightlightItem`))
  (bind _hightlightitem_2 (`self.HightlightItem`))
  (bind (_bblockinghit _binitialoverlap _time _distance _location _impactpoint _normal _impactnormal _physmat _hitactor) (`GameplayStatics.BreakHitResult` (`local.HitResult`)))
  (bind _camera (`/Game/Game/Blueprints/Characters/BP_CharacterBase.Camera` (`self.Owner`)))
  (bind _returnvalue (`SceneComponent.K2_GetComponentLocation` _camera))
  ;[1 1 1] Check in front of the player
  (bind (_outhit _returnvalue_2) (`KismetSystemLibrary.LineTraceSingle` _returnvalue (+ _returnvalue (* (`SceneComponent.GetForwardVector` _camera) (`self.GrabRange`))) "TraceTypeQuery1" false (`|MakeArray` (`self.Owner`) :!type "Actor Object Reference") "None" true (struct :`R` 1.0 :`G` 0.354083 :`B` 0.916096 :`A` 1.0) (struct :`G` 1.0 :`A` 1.0) 2.0))
  ;[1 1 1] Did we hit something.
  (bind _output_get (set `local.bHit` _returnvalue_2))
  (if _output_get
    ;[1 1 1] Is the last object in memory ?
    (bind _output_get_2 (set `local.HitResult` _outhit))
    (if (== (`self.HightlightItem`) (`.HitActor` (`GameplayStatics.BreakHitResult` _output_get_2)))
      ;[1 1 1] Still the same object so nothing changed
      (return)
      (else
        ;[1 1 1] We do not hightlight the last object in memory, so we reset it
        (`/Engine/EditorBlueprintResources/StandardMacros.IsValid` _hightlightitem
          (:`Is Valid`
            (`/Game/Game/Blueprints/Items/BP_GrabbableItem.ResetHightlight` _hightlightitem))
          (:`Is Not Valid`
            _))
        ;[1 1 1] Is the new object grabbable ?
        (if (`Actor.ActorHasTag` _hitactor (`self.GrabTag`))
          ;[1 1 1] Hightlight
          (bind _asbp_grabbable_item (cast `/Game/Game/Blueprints/Items/BP_GrabbableItem` _hitactor))
          (`/Game/Game/Blueprints/Items/BP_GrabbableItem.HightLightObject` _asbp_grabbable_item)
          (set `self.HightlightItem` _asbp_grabbable_item)
          (else
            (set `self.HightlightItem` null)))))
    (else
      (`/Engine/EditorBlueprintResources/StandardMacros.IsValid` _hightlightitem_2
        (:`Is Valid`
          (`/Game/Game/Blueprints/Items/BP_GrabbableItem.ResetHightlight` _hightlightitem_2)
          (set `self.HightlightItem` null))))))

(fn `StartAttack`
  (bind _hightlightitem (`self.HightlightItem`))
  (`parent.StartAttack`)
  (`/Engine/EditorBlueprintResources/StandardMacros.IsValid` (`self.GrabbedObject`)
    (:`Is Valid`
      ;[1 1 1] Throw object in hand
      (`/Game/Game/Blueprints/Items/BP_GrabbableItem.OnLauch` (`self.GrabbedObject`))
      (`PhysicsHandleComponent.ReleaseComponent` (`self.Grabber`))
      (`PrimitiveComponent.AddImpulse` (`/Game/Game/Blueprints/Items/BP_GrabbableItem.Mesh` (`self.GrabbedObject`)) (* (`SceneComponent.GetForwardVector` (`/Game/Game/Blueprints/Characters/BP_CharacterBase.Camera` (`self.Owner`))) (`self.ThrowPower`)) "None" false)
      (set `self.GrabbedObject` null))
    (:`Is Not Valid`
      ;[1 1 1] Grab object in sight
      (`/Engine/EditorBlueprintResources/StandardMacros.IsValid` _hightlightitem
        (:`Is Valid`
          (`PhysicsHandleComponent.GrabComponentAtLocation` (`self.Grabber`) (`/Game/Game/Blueprints/Items/BP_GrabbableItem.Mesh` _hightlightitem) "None" (`Actor.K2_GetActorLocation` _hightlightitem))
          (set `self.GrabbedObject` (`self.HightlightItem`)))))))