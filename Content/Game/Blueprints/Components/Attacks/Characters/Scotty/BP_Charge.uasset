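; Scotty's charge attack component, which drives the owner forward along the capsule's facing while the attack is in use.
; Init receives the mesh, movement, trigger, Niagara and timeline references from outside.
; StartAttack hides the sword, sets charge speed, plays effects and activates the charge trigger; EndAttack reverses this and changes the timeline's play rate.
; Tick accumulates a charge timer, but reaching its maximum triggers nothing here.
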(event `Init`
  (params (ChargeTriggerComponent :type "/Game/Game/Blueprints/Characters/Scotty/BP_ScottyChargeTrigger Object Reference") (ChargeNiagara :type "NiagaraComponent Object Reference") (MovementComponent :type "CharacterMovementComponent Object Reference") (SwordMesh :type "StaticMeshComponent Object Reference") (CapsuleComponent :type "CapsuleComponent Object Reference") (ChargeTimeline :type "TimelineComponent Object Reference"))
  (set `self.ChargeComponent` ChargeTriggerComponent)
  (set `self.ChargeNiagara` ChargeNiagara)
  (set `self.MovementComponent` MovementComponent)
  (set `self.Sword` SwordMesh)
  (set `self.CapsuleComponent` CapsuleComponent)
  (set `self.Charge Timeline` ChargeTimeline))

(event `self.ReceiveTick`
  (params (DeltaSeconds :type "Float (single-precision)"))
  (`self.UpdateCharge` DeltaSeconds))

(fn `EndAttack`
  (bind _sword (`self.Sword`))
  (`parent.EndAttack`)
  (`|ExecutionSequence`
    (:`then_0`
      ;[1 1 1] Disable Sword
      (`SceneComponent.SetHiddenInGame` _sword false false)
      (`PrimitiveComponent.SetCollisionEnabled` _sword "QueryOnly"))
    (:`then_1`
      ;[1 1 1] Set Speed
      (set `CharacterMovementComponent.MaxWalkSpeed` 300.0 (`self.MovementComponent`)))
    (:`then_2`
      ;[1 1 1] VFX
      (`TimelineComponent.SetPlayRate` (`self.Charge Timeline`) 2.5)
      (`self.Deactivate` (`self.ChargeNiagara`)))
    (:`then_3`
      ;[1 1 1] Reset
      (set `self.ChargeCurrentTimer` 0.0))
    (:`then_4`
      ;[1 1 1] Deactivate trigger
      (`/Game/Game/Blueprints/Characters/Scotty/BP_ScottyChargeTrigger.Deactivate` (`self.ChargeComponent`)))))

(fn `StartAttack`
  (bind _sword (`self.Sword`))
  (`parent.StartAttack`)
  (`|ExecutionSequence`
    (:`then_0`
      ;[1 1 1] Hide Sword
      (`SceneComponent.SetHiddenInGame` _sword true false)
      (`PrimitiveComponent.SetCollisionEnabled` _sword "NoCollision"))
    (:`then_1`
      ;[1 1 1] Speed Management
      (set `CharacterMovementComponent.MaxWalkSpeed` (`self.ChargeSpeed`) (`self.MovementComponent`)))
    (:`then_2`
      ;[1 1 1] Play Effects
      (`self.Activate` (`self.ChargeNiagara`) false)
      (`GameplayStatics.SpawnSoundAttached` (`self.ChargeSound`) (`self.CapsuleComponent`) "None" (0.0 0.0 0.0) (struct) "KeepRelativeOffset" false (`self.ChargeSoundVolumeMultiplier`) 1.0 0.0 null null))
    (:`then_3`
      ;[1 1 1] Activate charge collider
      (`/Game/Game/Blueprints/Characters/Scotty/BP_ScottyChargeTrigger.Activate` (`self.ChargeComponent`)))))

(fn `UpdateCharge`
  (params (Dt :type "Float (double-precision)"))
  (if (`self.IsInUse`)
    (`Pawn.AddMovementInput` (`self.Owner`) (`SceneComponent.GetForwardVector` (`self.CapsuleComponent`)) 1.0 false)
    (bind _output_get (set `self.ChargeCurrentTimer` (+ (`self.ChargeCurrentTimer`) Dt)))
    (if (>= _output_get (`self.ChargeMaxTimer`))
      _)))