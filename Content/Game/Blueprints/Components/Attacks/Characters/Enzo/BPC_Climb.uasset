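; Climb ability for the character Enzo, built as an attack component that lifts the owner up surfaces tagged Climbable.
; Starting it runs a camera-channel line trace from the capsule to a supplied end point to check for a climbable hit.
; Each tick repeats the trace, sets the default land movement to Flying and applies a small upward launch.
; Losing the surface or reaching the maximum climb time ends the attack and restores Walking.
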(event `self.ReceiveTick`
  (params (DeltaSeconds :type "Float (single-precision)"))
  (bind _owner (`self.Owner`))
  (`parent.ReceiveTick` DeltaSeconds)
  (if (`self.CanClimb`)
    (bind _returnvalue (`self.CheckForClimbableInSight`))
    (bind _output_get (set `self.CanClimb` _returnvalue))
    (if _output_get
      (bind _output_get_2 (set `self.ClimbTime` (+ (`self.ClimbTime`) DeltaSeconds)))
      (`KismetSystemLibrary.PrintString` (`KismetStringLibrary.Conv_DoubleToString` _output_get_2))
      (if (>= _output_get_2 (`self.MaxClimbTime`))
        (`self.EndAttack`)
        (else
          (set `CharacterMovementComponent.DefaultLandMovementMode` "MOVE_Flying" (`Character.CharacterMovement` _owner))
          (`Character.LaunchCharacter` _owner (0.0 0.0 20.0) false false)))
      (else
        (`self.EndAttack`)))))

(event `Init`
  (params (LineEndLocation :type "SceneComponent Object Reference") (EnzoCaps :type "CapsuleComponent Object Reference") (`Enzo Movement` :type "CharacterMovementComponent Object Reference"))
  (set `self.Line End Location` LineEndLocation)
  (set `self.Enzo Caps` EnzoCaps)
  (set `self.Enzo Movement` `Enzo Movement`))

(fn `CheckForClimbableInSight`
  (returns (ReturnValue :type Boolean))
  (bind _outhit (`KismetSystemLibrary.LineTraceSingle` :`Start` (`SceneComponent.K2_GetComponentLocation` (`self.Enzo Caps`)) :`End` (`SceneComponent.K2_GetComponentLocation` (`self.Line End Location`)) :`TraceChannel` "TraceTypeQuery2" :`DrawDebugType` "ForDuration"))
  (if (`GameplayStatics.BreakHitResult` _outhit)
    (return (`Actor.ActorHasTag` (`.HitActor` (`GameplayStatics.BreakHitResult` _outhit)) "Climbable"))))

(fn `EndAttack`
  (`parent.EndAttack`)
  (set `self.CanClimb` false)
  (set `self.ClimbTime` 0.0)
  (set `CharacterMovementComponent.DefaultLandMovementMode` "MOVE_Walking" (`Character.CharacterMovement` (`self.Owner`))))

(fn `StartAttack`
  (`parent.StartAttack`)
  (bind _returnvalue (`self.CheckForClimbableInSight`))
  (set `self.CanClimb` _returnvalue))

(fn `TryStartAttack`
  (if (not (`self.IsInUse`))
    (`self.StartAttack`)
    (`self.ExecuteAttack`)))