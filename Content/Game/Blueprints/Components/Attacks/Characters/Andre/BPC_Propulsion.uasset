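; Attack component for the character Andre that launches its owner vertically when the attack ends.
; The attack only starts while the owner is not falling, then resets its timer and deactivates movement.
; On end, it restores movement and calls LaunchCharacter with an upward force scaled by elapsed time over the attack's maximum duration, clamped to the maximum propulsion force.
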(fn `EndAttack`
  (`parent.EndAttack`)
  (`/Game/Game/Blueprints/Characters/BP_CharacterBase.ActivateMovement` (`self.Owner`))
  (`self.PropulsePlayer` (`KismetMathLibrary.FClamp` (`KismetMathLibrary.Lerp` 0.0 (`self.MaxPropulsionForce`) (/ (`self.TimeElapsed`) (`self.AttackMaxDuration`))) 0.0 (`self.MaxPropulsionForce`))))

(fn `PropulsePlayer`
  (params (VerticalForce :type "Float (double-precision)"))
  (`KismetSystemLibrary.PrintString` "Propulse player")
  (`Character.LaunchCharacter` (`self.Owner`) (`KismetMathLibrary.MakeVector` 0.0 0.0 VerticalForce) false false)
  (return))

(fn `StartAttack`
  (set `self.TimeElapsed` 0.0)
  (`parent.StartAttack`)
  (`/Game/Game/Blueprints/Characters/BP_CharacterBase.DeactivateMovement` (`self.Owner`)))

(fn `TryStartAttack`
  (if (not (`NavMovementComponent.IsFalling` (`Character.CharacterMovement` (`self.Owner`))))
    (`parent.TryStartAttack`)))