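; BPC_Dash is an attack component, filed under the character Andre, that dashes its owner a set distance along its movement direction or facing.
; Starting the attack disables input and gravity and picks the direction; execution hides the mesh, activates the supplied VFX and starts a looping frame-delta timer.
; Dash movement uses swept VInterpTo steps toward the target.
; A blocking hit or arrival ends it, restoring visibility, input and gravity and zeroing vertical velocity.
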(event `Initialize`
  (params (DashVFX :type "NiagaraComponent Object Reference"))
  (set `self.DashVFX` DashVFX))

(event `self.ExecuteAttack`
  (bind _returnvalue (`KismetSystemLibrary.K2_SetTimerDelegate` (`|CreateDelegate` :!event `Dash`) (`GameplayStatics.GetWorldDeltaSeconds`) true))
  (set `self.DashTimer` _returnvalue)
  (`SceneComponent.SetVisibility` (`Character.Mesh` (`self.Owner`)) false false)
  (`self.ActivateVFX`))

(event `Dash`
  (set `self.PredicatedLocation` (+ (* (`self.DashDirection`) (`self.DashDistance`)) (`self.BaseLocation`)))
  (bind _sweephitresult (`Actor.K2_SetActorLocation` (`self.Owner`) (`KismetMathLibrary.VInterpTo` (`Actor.K2_GetActorLocation` (`self.Owner`)) (`self.PredicatedLocation`) (`GameplayStatics.GetWorldDeltaSeconds`) (`self.DashSpeed`)) true false))
  (if (or (`GameplayStatics.BreakHitResult` _sweephitresult) (== (`KismetMathLibrary.Conv_VectorToVector2D` (`self.PredicatedLocation`)) (`KismetMathLibrary.Conv_VectorToVector2D` (`Actor.K2_GetActorLocation` (`self.Owner`))) :`ErrorTolerance` 100.0))
    (`self.EndAttack`)))

(fn `ActivateVFX`
  (bind _dashvfx (`self.DashVFX`))
  (`/Engine/EditorBlueprintResources/StandardMacros.IsValid` _dashvfx
    (:`Is Valid`
      (`self.Activate` _dashvfx false)
      (return))))

(fn `DeactivateVFX`
  (bind _dashvfx (`self.DashVFX`))
  (`/Engine/EditorBlueprintResources/StandardMacros.IsValid` _dashvfx
    (:`Is Valid`
      (`self.Deactivate` _dashvfx)
      (return))))

(fn `DetermineDashDirection`
  (locals (BaseVelocity :type "Vector2D Structure"))
  (if (`self.IsVelocityBased`)
    (bind _output_get (set `local.BaseVelocity` (`KismetMathLibrary.Conv_VectorToVector2D` (`KismetMathLibrary.Vector_Normal2D` (`MovementComponent.Velocity` (`Character.CharacterMovement` (`self.Owner`)))))))
    (if (`KismetMathLibrary.IsZero2D` _output_get)
      ;[1 1 1] Dash forward
      (set `self.DashDirection` (`KismetMathLibrary.Conv_VectorToVector2D` (`Actor.GetActorForwardVector` (`self.Owner`))))
      (return)
      (else
        ;[1 1 1] Dash depending the velocity
        (set `self.DashDirection` (`local.BaseVelocity`))
        (return)))
    (else
      ;[1 1 1] Dash forward
      (set `self.DashDirection` (`KismetMathLibrary.Conv_VectorToVector2D` (`Actor.GetActorForwardVector` (`self.Owner`))))
      (return))))

(fn `EndAttack`
  (bind _dashtimer (`self.DashTimer`))
  (bind _charactermovement (`Character.CharacterMovement` (`self.Owner`)))
  (`|ExecutionSequence`
    (:`then_0`
      (if (`KismetSystemLibrary.K2_IsValidTimerHandle` _dashtimer)
        (`KismetSystemLibrary.K2_ClearAndInvalidateTimerHandle` _dashtimer)))
    (:`then_1`
      (`SceneComponent.SetVisibility` (`Character.Mesh` (`self.Owner`)) true false)
      (`self.DeactivateVFX`)
      (`Actor.EnableInput` (`self.Owner`) (`GameplayStatics.GetPlayerController` 0))
      (`/Game/Game/Blueprints/Characters/BP_CharacterBase.SetGravityScale` (`self.Owner`) (`self.BaseGravityScale`))
      (set `MovementComponent.Velocity` (`KismetMathLibrary.Conv_Vector2DToVector` (`KismetMathLibrary.Conv_VectorToVector2D` (`MovementComponent.Velocity` _charactermovement))) _charactermovement)
      (`parent.EndAttack`))))

(fn `OnRelease`)

(fn `StartAttack`
  (`parent.StartAttack`)
  (set `self.BaseLocation` (`Actor.K2_GetActorLocation` (`self.Owner`)))
  (`self.DetermineDashDirection`)
  (`Actor.DisableInput` (`self.Owner`) (`GameplayStatics.GetPlayerController` 0))
  (set `self.BaseGravityScale` (`CharacterMovementComponent.GravityScale` (`Character.CharacterMovement` (`self.Owner`))))
  (`/Game/Game/Blueprints/Characters/BP_CharacterBase.SetGravityScale` (`self.Owner`) 0.0))