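; BPC_HealthBar is a health bar component that drives a WB_Health widget.
; BindWidget takes a WidgetComponent, casts its user widget to WB_Health and caches the reference.
; TryUpdateWidget uses that reference, if valid, to set the fill percent from current over max health and tint it by interpolating between the empty and full colors.
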(fn `BindWidget`
  (params (`Widget Component` :type "WidgetComponent Object Reference"))
  (`/Engine/EditorBlueprintResources/StandardMacros.IsValid` `Widget Component`
    (:`Is Valid`
      (bind _aswb_health (cast `/Game/Game/Blueprints/UI/WB_Health` (`WidgetComponent.GetUserWidgetObject` `Widget Component`)))
      (set `self.HealthWidget` _aswb_health))))

(fn `TryUpdateWidget`
  (params (CurrentHealth :type "Float (double-precision)") (MaxHealth :type "Float (double-precision)"))
  (bind _healthwidget (`self.HealthWidget`))
  (`/Engine/EditorBlueprintResources/StandardMacros.IsValid` _healthwidget
    (:`Is Valid`
      (bind _output_get (set `/Game/Game/Blueprints/UI/WB_Health.HealthPercent` (/ CurrentHealth MaxHealth) _healthwidget))
      (set `/Game/Game/Blueprints/UI/WB_Health.Color` (`KismetMathLibrary.LinearColorLerp` (`self.ColorEmpty`) (`self.ColorFull`) _output_get) _healthwidget))))