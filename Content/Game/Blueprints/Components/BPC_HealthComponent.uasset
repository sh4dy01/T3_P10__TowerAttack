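; BPC_HealthComponent is a health component that tracks Health for its owner and signals death through an OnDeath delegate.
; Health starts at MaxHealth on BeginPlay, is exposed through GetHealth, and is lowered by ApplyDamage within zero and MaxHealth.
; The death check recomputes the clamped subtraction after Health is set, so OnDeath fires when the new Health minus Damage again reaches zero or below.
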(event `self.ReceiveBeginPlay`
  (set `self.Health` (`self.MaxHealth`)))

(fn `ApplyDamage`
  (params (Damage :type "Float (double-precision)"))
  (bind _returnvalue (`KismetMathLibrary.FClamp` (- (`self.Health`) Damage) 0.0 (`self.MaxHealth`)))
  (set `self.Health` _returnvalue)
  (if (<= _returnvalue 0.0)
    (`self.OnDeathDelegate`)))

(fn `GetHealth`
  (returns (Health :type "Float (double-precision)"))
  (return (`self.Health`)))