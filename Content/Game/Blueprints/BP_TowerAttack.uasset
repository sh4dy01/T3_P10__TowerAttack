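; BP_TowerAttack is game-mode-style setup logic that prepares the player's character switching when play begins.
; On BeginPlay it caches the first BP_BasePlayerController, then spawns a BP_CharacterSwitcher at the player start.
; It hands the switcher to the controller, binds to its OnCharacterSwitch event and initializes it with the first character.
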(event `self.ReceiveBeginPlay`
  (`|ExecutionSequence`
    (:`then_0`
      (bind _asbp_base_player_controller (cast `/Game/Game/Blueprints/BP_BasePlayerController` (`GameplayStatics.GetPlayerController` 0)))
      (set `self.PlayerController` _asbp_base_player_controller))
    (:`then_1`
      (bind _returnvalue (`|SpawnActorFromClass` "/Game/Game/Blueprints/BP_CharacterSwitcher.BP_CharacterSwitcher_C" (`self.GetTransform` (`self.K2_FindPlayerStart` null)) "Undefined" "MultiplyWithRoot" null null))
      (bind _output_get (set `self.CharacterSwitch` _returnvalue))
      (bind _output_get_2 (set `/Game/Game/Blueprints/BP_BasePlayerController.CharacterSwitcher` _output_get (`self.PlayerController`)))
      (add `/Game/Game/Blueprints/BP_CharacterSwitcher.OnCharacterSwitch` _output_get_2 (`|CreateDelegate` (`self.PlayerController`) :!event `UpdateControlledCharacter`)))
    (:`then_2`
      (`/Game/Game/Blueprints/BP_CharacterSwitcher.InitializeWithCharacter` (`self.CharacterSwitch`) 0))))

(fn `UserConstructionScript`)