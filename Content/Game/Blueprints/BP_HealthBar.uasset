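; BP_HealthBar is an actor Blueprint that pairs a health component with a world-space health bar.
; On BeginPlay it subscribes to the component's OnHealthUpdated event and calls BindWidget on the bar.
; Each Tick it rotates the bar to face player 0's character location, rather than the camera.
; Init passes MaxHealth to the health component, while GetHealthComponent has no value wired to its return.
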(event `self.ReceiveBeginPlay`
  (add `/Game/Game/Blueprints/Components/BPC_HealthComponent.OnHealthUpdated` (`self.HealthComponent`) (`|CreateDelegate` (`self.HealthBar`) :!event `TryUpdateWidget`))
  (`/Game/Game/Blueprints/Components/BPC_HealthBar.BindWidget` (`self.HealthBar`) (`self.Health Bar`)))

(event `self.ReceiveTick`
  (params (DeltaSeconds :type "Float (single-precision)"))
  (`SceneComponent.K2_SetWorldRotation` (`self.Health Bar`) (`KismetMathLibrary.FindLookAtRotation` (`SceneComponent.K2_GetComponentLocation` (`self.Health Bar`)) (`self.K2_GetActorLocation` (`GameplayStatics.GetPlayerCharacter` 0))) false false))

(fn `GetHealthComponent`
  (returns (`Health Component` :type "/Game/Game/Blueprints/Components/BPC_HealthComponent Object Reference"))
  (return null))

(fn `Init`
  (params (MaxHealth :type "Float (double-precision)"))
  (`/Game/Game/Blueprints/Components/BPC_HealthComponent.Init` (`self.HealthComponent`) MaxHealth))

(fn `UserConstructionScript`)