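; BP_ShieldTowerSystem groups two shield towers and a wall, removing the wall once the towers are destroyed.
; On BeginPlay it binds to both child-actor towers' destroyed delegates and caches the wall.
; Each destroyed event decrements NumberOfTowers; at zero it calls NukeSelf on the wall, then destroys itself.
; An unconnected Construction Script graph for spawning the wall and a variable tower count never runs.
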(event `self.ReceiveBeginPlay`
  (bind _asbp_shield_tower (cast `/Game/Game/Blueprints/Towers/DefenseTower/BP_ShieldTower` (`ChildActorComponent.ChildActor` (`self.FirstTower`))))
  (add `/Game/Game/Blueprints/Towers/BP_TowerBase.OnTowerDestroyedDelegate` _asbp_shield_tower (`|CreateDelegate` :!event `OnTowerDestroyed`))
  (bind _asbp_shield_tower_2 (cast `/Game/Game/Blueprints/Towers/DefenseTower/BP_ShieldTower` (`ChildActorComponent.ChildActor` (`self.SecondTower`))))
  (add `/Game/Game/Blueprints/Towers/BP_TowerBase.OnTowerDestroyedDelegate` _asbp_shield_tower_2 (`|CreateDelegate` :!event `OnTowerDestroyed`))
  (bind _asbp_wall (cast `/Game/Game/Blueprints/Towers/DefenseTower/BP_Wall` (`ChildActorComponent.ChildActor` (`self.Wall`))))
  (set `self.WallRef` _asbp_wall))

(event `OnTowerDestroyed`
  (bind _result (`/Engine/EditorBlueprintResources/StandardMacros.DecrementInt` (`self.NumberOfTowers`))
    (:`  `
      (if (<= _result 0)
        (`/Game/Game/Blueprints/Towers/DefenseTower/BP_Wall.NukeSelf` (`self.WallRef`))
        (`self.K2_DestroyActor`)))))

(fn `UserConstructionScript`)