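; Base tower actor that can take damage and be destroyed.
; On BeginPlay it initializes a child-actor BP_HealthBar with MaxHealth, borrows its HealthComponent and binds death and damage events.
; Incoming damage is forwarded to that component.
; On death it broadcasts OnTowerDestroyed, prints a message, then, if the monument mesh is valid, disables its collision and destroys itself.
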(event `self.ReceiveBeginPlay`
  (`|ExecutionSequence`
    (:`then_0`
      (bind _asbp_health_bar (cast `/Game/Game/Blueprints/BP_HealthBar` (`ChildActorComponent.ChildActor` (`self.HealthBar`))))
      (`/Game/Game/Blueprints/BP_HealthBar.Init` _asbp_health_bar (`self.MaxHealth`))
      (bind _output_get (set `self.HealthComponent` (`/Game/Game/Blueprints/BP_HealthBar.HealthComponent` _asbp_health_bar)))
      (add `/Game/Game/Blueprints/Components/BPC_HealthComponent.OnDeathDelegate` _output_get (`|CreateDelegate` :!event `OnDeath`)))
    (:`then_1`
      (add `self.OnTakeAnyDamage` (`|CreateDelegate` :!event `OnTakeDamage`)))))

(event `OnDeath`
  (bind _sm_monument_06 (`self.SM_Monument_06`))
  (`self.OnTowerDestroyedDelegate`)
  (`KismetSystemLibrary.PrintString` "Tower Destroyed")
  (`/Engine/EditorBlueprintResources/StandardMacros.IsValid` _sm_monument_06
    (:`Is Valid`
      (`PrimitiveComponent.SetCollisionEnabled` _sm_monument_06 "NoCollision")
      (`self.NukeSelf`))))

(event `OnTakeDamage` :!signature `self.OnTakeAnyDamage`
  (params (DamagedActor :type "Actor Object Reference") (Damage :type "Float (single-precision)") (DamageType :type "DamageType Object Reference") (InstigatedBy :type "Controller Object Reference") (DamageCauser :type "Actor Object Reference"))
  (`/Engine/EditorBlueprintResources/StandardMacros.IsValid` (`self.HealthComponent`)
    (:`Is Valid`
      (`/Game/Game/Blueprints/Components/BPC_HealthComponent.ApplyDamage` (`self.HealthComponent`) Damage))))

(fn `NukeSelf`
  (`self.K2_DestroyActor`))

(fn `UserConstructionScript`)