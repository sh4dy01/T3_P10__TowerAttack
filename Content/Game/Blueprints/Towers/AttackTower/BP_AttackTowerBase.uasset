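; Base attack tower that detects characters entering or leaving its AttackRange and changes its particle effect to match.
; Overlaps with BP_CharacterBase fire in-range and out-of-range delegates, bound at BeginPlay, with empty OnPlayerInRange and OnPlayerOutOfRange functions present as stubs.
; A shared helper, NewFunction, pushes Normal or Attack parameter sets to the particle system, applying Normal at construction and on exit, Attack on entry.
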(event `self.ReceiveBeginPlay`
  (`parent.ReceiveBeginPlay`)
  (add `self.OnPlayerInAttackRangeDelegate` (`|CreateDelegate` :!event `OnPlayerInRange`))
  (add `self.OnPlayerOutOfAttackRangeDelegate` (`|CreateDelegate` :!event `OnPlayerOutOfRange`)))

(event `self.AttackRange.OnComponentBeginOverlap`
  (params (OverlappedComponent :type "PrimitiveComponent Object Reference") (OtherActor :type "Actor Object Reference") (OtherComp :type "PrimitiveComponent Object Reference") (OtherBodyIndex :type Integer) (bFromSweep :type Boolean) (SweepResult :type "HitResult Structure (by ref)"))
  (bind _asbp_character_base (cast `/Game/Game/Blueprints/Characters/BP_CharacterBase` OtherActor))
  (bind _output_get (set `self.PlayerRef` _asbp_character_base))
  (`self.OnPlayerInAttackRangeDelegate` _output_get)
  (`self.NewFunction` (`self.AttackParticleColor`) (`self.AttackLifetime`) (`self.AttackMinVelocity`) (`self.AttackMaxVelocity`) (`self.AttackSpawnRate`)))

(event `self.AttackRange.OnComponentEndOverlap`
  (params (OverlappedComponent :type "PrimitiveComponent Object Reference") (OtherActor :type "Actor Object Reference") (OtherComp :type "PrimitiveComponent Object Reference") (OtherBodyIndex :type Integer))
  (bind _asbp_character_base (cast `/Game/Game/Blueprints/Characters/BP_CharacterBase` OtherActor))
  (`self.OnPlayerOutOfAttackRangeDelegate` _asbp_character_base)
  (`self.NewFunction` (`self.NormalParticleColor`) (`self.NormalLifetime`) (`self.NormalMinVelocity`) (`self.NormalMaxVelocity`) (`self.NormalSpawnRate`)))

(fn `NewFunction`
  (params (Color :type "LinearColor Structure (by ref)") (Lifetime :type "Float (single-precision)") (MinVelocity :type "Float (single-precision)") (MaxVelocity :type "Float (single-precision)") (SpawnRate :type "Float (single-precision)"))
  (`|ExecutionSequence`
    (:`then_0`
      (`NiagaraComponent.SetVariableLinearColor` (`self.ParticleSystem`) "ParticleColor" Color))
    (:`then_1`
      (`NiagaraComponent.SetVariableFloat` (`self.ParticleSystem`) "Lifetime" Lifetime))
    (:`then_2`
      (`NiagaraComponent.SetVariableFloat` (`self.ParticleSystem`) "MinVelocity" MinVelocity))
    (:`then_3`
      (`NiagaraComponent.SetVariableFloat` (`self.ParticleSystem`) "MaxVelocity" MaxVelocity))
    (:`then_4`
      (`NiagaraComponent.SetVariableFloat` (`self.ParticleSystem`) "SpawnRate" SpawnRate)
      (return))))

(fn `OnPlayerInRange`
  (params (Player :type "/Game/Game/Blueprints/Characters/BP_CharacterBase Object Reference")))

(fn `OnPlayerOutOfRange`
  (params (Player :type "/Game/Game/Blueprints/Characters/BP_CharacterBase Object Reference")))

(fn `UserConstructionScript`
  (`parent.UserConstructionScript`)
  (`self.NewFunction` (`self.NormalParticleColor`) (`self.NormalLifetime`) (`self.NormalMinVelocity`) (`self.NormalMaxVelocity`) (`self.NormalSpawnRate`)))