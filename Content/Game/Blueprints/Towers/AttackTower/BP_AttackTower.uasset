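; BP_AttackTower is a tower that fires homing projectiles at the player while they are in range.
; Entering range starts a looping timer at the FireRate interval, and leaving range clears it.
; Each shot spawns a BP_AttackTowerProjectile at AttackPoint, aimed at PlayerRef, and sets the player's Scene component as its homing target.
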(fn `FireProjectile`
  (locals (NormalizeTolerence :type "Float (single-precision)" :default 0.0001))
  (bind _returnvalue (`SceneComponent.K2_GetComponentLocation` (`self.AttackPoint`)))
  (bind _playerref (`self.PlayerRef`)
    (:`then`
      (bind _returnvalue_2 (`|SpawnActorFromClass` "/Game/Game/Blueprints/Actors/Projectiles/BP_AttackTowerProjectile.BP_AttackTowerProjectile_C" (`KismetMathLibrary.MakeTransform` _returnvalue (`KismetMathLibrary.MakeRotFromX` (`KismetMathLibrary.Normal` (- (`self.K2_GetActorLocation` _playerref) _returnvalue) (`local.NormalizeTolerence`)))) "Undefined" "MultiplyWithRoot" null null))
      (set `ProjectileMovementComponent.HomingTargetComponent` (`/Game/Game/Blueprints/Characters/BP_CharacterBase.Scene` (`self.PlayerRef`)) (`/Game/Game/Blueprints/Actors/Projectiles/BP_Projectile.ProjectileMovement` _returnvalue_2)))
    (:`else`)))

(fn `OnPlayerInRange`
  (params (Player :type "/Game/Game/Blueprints/Characters/BP_CharacterBase Object Reference"))
  (bind _returnvalue (`KismetSystemLibrary.K2_SetTimer` null "FireProjectile" (/ 1.0 (`self.FireRate`)) true))
  (set `self.FireTimerHandle` _returnvalue))

(fn `OnPlayerOutOfRange`
  (params (Player :type "/Game/Game/Blueprints/Characters/BP_CharacterBase Object Reference"))
  (`KismetSystemLibrary.K2_ClearAndInvalidateTimerHandle` (`self.FireTimerHandle`)))

(fn `UserConstructionScript`
  (`parent.UserConstructionScript`))