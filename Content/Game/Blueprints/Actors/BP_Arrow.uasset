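; BP_Arrow is a physics-driven arrow projectile that launches itself along its forward vector on BeginPlay with an impulse on the Arrow component.
; Every tick, it applies a force at the Tail component's location equal to the Tail's linear velocity scaled by Drag.
; This velocity-proportional tail force acts like fletching, influencing orientation through physics instead of setting rotation directly.
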(event `self.ReceiveBeginPlay`
  (`PrimitiveComponent.AddImpulse` (`self.Arrow`) (* (`self.GetActorForwardVector`) (`self.Impulse`)) "None" false))

(event `self.ReceiveTick`
  (params (DeltaSeconds :type "Float (single-precision)"))
  (bind _tail (`self.Tail`))
  (bind _returnvalue (`PrimitiveComponent.GetPhysicsLinearVelocity` (`self.Tail`) "None"))
  (`PrimitiveComponent.AddForceAtLocation` _tail (* _returnvalue (`self.Drag`)) (`SceneComponent.K2_GetComponentLocation` _tail) "None"))

(fn `UserConstructionScript`)