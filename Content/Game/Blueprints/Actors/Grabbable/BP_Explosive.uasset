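; Grabbable explosive that, once launched, starts its fire effect, waits out a fuse delay, then explodes with particles and sound and destroys itself.
; Explode uses Chaos physics fields sized by the DamageZone sphere: radial falloff sets dynamic state and cluster strain to fracture structures, and a culled radial vector pushes the blocks outward.
; ApplyDamage is called without a target actor, and HandleExplosionOnActor is an empty stub.
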(event `self.OnLauch`
  (bind _returnvalue (`SceneComponent.K2_GetComponentLocation` (`self.Mesh`)))
  (`ActorComponent.Activate` (`self.Fire`) false)
  (`KismetSystemLibrary.Delay` (`self.TimeBeforeExplosion`))
  (`GameplayStatics.SpawnEmitterAtLocation` "/Game/StarterContent/Particles/P_Explosion.P_Explosion" _returnvalue (struct) (10.0 10.0 10.0))
  (`GameplayStatics.SpawnSoundAtLocation` "/Game/StarterContent/Audio/Explosion02.Explosion02" _returnvalue (struct) 1.0 1.0 0.0 null null)
  (`self.Explode`)
  (`self.K2_DestroyActor`))

(event `Explode`
  (bind _damagezone (`self.DamageZone`))
  (bind _returnvalue (`RadialFalloff.SetRadialFalloff` (`self.RadialFalloff`) (`self.ExplosionMagnitude`) 0.0 1.0 0.0 (`SphereComponent.GetScaledSphereRadius` _damagezone) (`SceneComponent.K2_GetComponentLocation` _damagezone) "Field_Falloff_Linear"))
  (`GameplayStatics.ApplyDamage` null 50.0 null self)
  (`FieldSystemComponent.ApplyPhysicsField` (`self.FieldSystemComponent`) true "Field_DynamicState" null _returnvalue)
  (`FieldSystemComponent.ApplyPhysicsField` (`self.FieldSystemComponent`) true "Field_ExternalClusterStrain" null _returnvalue)
  (`FieldSystemComponent.ApplyPhysicsField` (`self.FieldSystemComponent`) true "Field_LinearVelocity" null (`CullingField.SetCullingField` (`self.CullingField`) _returnvalue (`RadialVector.SetRadialVector` (`self.RadialVector`) (`self.ExplosionVelocityMagnitude`) (`SceneComponent.K2_GetComponentLocation` (`self.DamageZone`))) "Field_Culling_Outside")))

(fn `HandleExplosionOnActor`
  (params (DamagedActor :type "Actor Object Reference")))

(fn `UserConstructionScript`
  (`parent.UserConstructionScript`))