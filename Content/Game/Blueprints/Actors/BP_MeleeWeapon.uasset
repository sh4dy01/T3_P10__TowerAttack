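; Melee weapon actor that deals damage and shows hit effects during the owner's primary attack.
; Primary use start and end toggle the sword trail and the damage box's query collision.
; ApplyDamageToOtherActor hits once per attack via the attack component's HasAppliedDamage flag, picking falling-attack damage while the in-air montage plays, otherwise damage by combo index.
; Each hit spawns a Niagara effect at HitLocation.
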(fn `ApplyDamageToOtherActor`
  (params (DamagedActor :type "Actor Object Reference"))
  (bind _primaryattackref (`self.PrimaryAttackRef`))
  (bind _primaryattackref_2 (`self.PrimaryAttackRef`))
  (if (not (`/Game/Game/Blueprints/Components/Attacks/Base/BPC_ComboAttack.HasAppliedDamage` (`self.PrimaryAttackRef`)))
    (bind _returnvalue (`/Game/Game/Blueprints/Components/Attacks/Base/BPC_ComboAttack.IsMontagePlaying` _primaryattackref_2 (`/Game/Game/Blueprints/Components/Attacks/Base/BPC_ComboAttack.InAirAttackMontage` _primaryattackref_2)))
    (if _returnvalue
      (`GameplayStatics.ApplyDamage` DamagedActor (`/Game/Game/Blueprints/Components/Attacks/Base/BPC_ComboAttack.FallingAttackDamage` (`self.PrimaryAttackRef`)))
      (set `/Game/Game/Blueprints/Components/Attacks/Base/BPC_ComboAttack.HasAppliedDamage` true (`self.PrimaryAttackRef`))
      (`/Game/Game/Blueprints/Characters/Juan/BP_Hammer.SpawnHitParticles`)
      (`KismetSystemLibrary.PrintString` "Hit" true true (struct :`R` 1.0 :`G` 0.09424 :`A` 1.0))
      (else
        (`GameplayStatics.ApplyDamage` DamagedActor (`BlueprintMapLibrary.Map_Find` (`/Game/Game/Blueprints/Components/Attacks/Base/BPC_ComboAttack.Damages` _primaryattackref) (`/Game/Game/Blueprints/Components/Attacks/Base/BPC_ComboAttack.ComboIndex` _primaryattackref)))
        (set `/Game/Game/Blueprints/Components/Attacks/Base/BPC_ComboAttack.HasAppliedDamage` true (`self.PrimaryAttackRef`))
        (`/Game/Game/Blueprints/Characters/Juan/BP_Hammer.SpawnHitParticles`)
        (`KismetSystemLibrary.PrintString` "Hit" true true (struct :`R` 1.0 :`G` 0.09424 :`A` 1.0))))))

(fn `OnPrimaryEnded`
  (`ActorComponent.Deactivate` (`self.SwordTrail`))
  (`PrimitiveComponent.SetCollisionEnabled` (`self.WeaponDamageBox`) "NoCollision")
  (return))

(fn `OnPrimaryUsed`
  (`ActorComponent.Activate` (`self.SwordTrail`) false)
  (`PrimitiveComponent.SetCollisionEnabled` (`self.WeaponDamageBox`) "QueryOnly")
  (return))

(fn `SpawnHitParticles`
  (`NiagaraFunctionLibrary.SpawnSystemAtLocation` "/Game/Game/Art/Particles/NS_Hit.NS_Hit" (`SceneComponent.K2_GetComponentLocation` (`self.HitLocation`))))

(fn `UserConstructionScript`)