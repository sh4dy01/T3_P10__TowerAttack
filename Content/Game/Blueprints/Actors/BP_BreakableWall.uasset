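; BP_BreakableWall is a breakable wall actor that uses a Chaos physics field to change object state when a trigger touches it.
; When an actor tagged ChaosTrigger begins overlapping the Collider, the FieldSystemComponent issues a dynamic state field command.
; The command applies the FieldState variable as a uniform integer, culled outside a box falloff built from the Collider's world transform.
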(event `self.Collider.OnComponentBeginOverlap`
  (params (OverlappedComponent :type "PrimitiveComponent Object Reference") (OtherActor :type "Actor Object Reference") (OtherComp :type "PrimitiveComponent Object Reference") (OtherBodyIndex :type Integer) (bFromSweep :type Boolean) (SweepResult :type "HitResult Structure (by ref)"))
  (if (`self.ActorHasTag` OtherActor "ChaosTrigger")
    (`FieldSystemComponent.AddFieldCommand` (`self.FieldSystemComponent`) true "Field_DynamicState" null (`CullingField.SetCullingField` (`self.CullingField`) (`BoxFalloff.SetBoxFalloff` (`self.BoxFalloff`) 1.0 0.0 1.0 0.0 (`SceneComponent.K2_GetComponentToWorld` (`self.Collider`)) "Field_FallOff_None") (`UniformInteger.SetUniformInteger` (`self.UniformInteger`) (`KismetMathLibrary.Conv_ByteToInt` (`self.FieldState`))) "Field_Culling_Outside"))))

(fn `UserConstructionScript`)