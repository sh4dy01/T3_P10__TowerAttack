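; BP_LavaFan is a fan actor whose capsule volume lifts any BP_CharacterBase that enters it.
; On overlap it saves the character's gravity scale, inverts gravity, replaces velocity with a small upward one and adds a slight downward force once.
; On exit it restores the saved scale, which is held in one variable shared by all overlapping characters.
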(event `self.Capsule.OnComponentBeginOverlap`
  (params (OverlappedComponent :type "PrimitiveComponent Object Reference") (OtherActor :type "Actor Object Reference") (OtherComp :type "PrimitiveComponent Object Reference") (OtherBodyIndex :type Integer) (bFromSweep :type Boolean) (SweepResult :type "HitResult Structure (by ref)"))
  (bind _asbp_character_base (cast `/Game/Game/Blueprints/Characters/BP_CharacterBase` OtherActor))
  (bind _charactermovement (`Character.CharacterMovement` _asbp_character_base))
  (set `self.PreviousGravityScale` (`CharacterMovementComponent.GravityScale` _charactermovement))
  (set `CharacterMovementComponent.GravityScale` -1.0 _charactermovement)
  (set `MovementComponent.Velocity` (0.0 0.0 100.0) _charactermovement)
  (`CharacterMovementComponent.AddForce` _charactermovement (0.0 0.0 -100.0)))

(event `self.Capsule.OnComponentEndOverlap`
  (params (OverlappedComponent :type "PrimitiveComponent Object Reference") (OtherActor :type "Actor Object Reference") (OtherComp :type "PrimitiveComponent Object Reference") (OtherBodyIndex :type Integer))
  (bind _asbp_character_base (cast `/Game/Game/Blueprints/Characters/BP_CharacterBase` OtherActor))
  (set `CharacterMovementComponent.GravityScale` (`self.PreviousGravityScale`) (`Character.CharacterMovement` _asbp_character_base)))

(event `CustomEvent`
  (params (OverlappedComponent :type "PrimitiveComponent Object Reference") (OtherActor :type "Actor Object Reference") (OtherComp :type "PrimitiveComponent Object Reference") (OtherBodyIndex :type Integer)))

(fn `UserConstructionScript`)