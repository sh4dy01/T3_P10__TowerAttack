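; BP_Lava is a lava hazard actor that punishes characters and destroys any other actor overlapping its static mesh.
; A character hitting it with vertical speed above a threshold in either direction takes HeroDamage through its health component and respawns at a safe zone.
; A slower vertical contact restarts the level through a console command.
; SetSpeed lets callers change the max speed of the lava's VerticalMovement component.
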(event `self.StaticMesh.OnComponentBeginOverlap`
  (params (OverlappedComponent :type "PrimitiveComponent Object Reference") (OtherActor :type "Actor Object Reference") (OtherComp :type "PrimitiveComponent Object Reference") (OtherBodyIndex :type Integer) (bFromSweep :type Boolean) (SweepResult :type "HitResult Structure (by ref)"))
  (bind _asbp_character_base (cast `/Game/Game/Blueprints/Characters/BP_CharacterBase` OtherActor)
    (:`then`
      (bind (_returnvalue_x _returnvalue_y _returnvalue_z) (`KismetMathLibrary.BreakVector` (`CharacterMovementComponent.GetLastUpdateVelocity` (`Character.CharacterMovement` _asbp_character_base))))
      (if (> (`KismetMathLibrary.Abs` _returnvalue_z) 200.0)
        (`/Game/Game/Blueprints/Components/BPC_HealthComponent.ApplyDamage` (`/Game/Game/Blueprints/Characters/BP_CharacterBase.HealthComponent` _asbp_character_base) (`self.HeroDamage`))
        (`/Game/Game/Blueprints/Characters/BP_CharacterBase.RespawnPlayerToSafeZone` _asbp_character_base)
        (else
          (`KismetSystemLibrary.ExecuteConsoleCommand` "RestartLevel" null))))
    (:`CastFailed`
      (`self.K2_DestroyActor` OtherActor))))

(fn `SetSpeed`
  (params (NewSpeed :type "Float (double-precision)"))
  (set `FloatingPawnMovement.MaxSpeed` NewSpeed (`self.VerticalMovement`))
  (return))

(fn `UserConstructionScript`)