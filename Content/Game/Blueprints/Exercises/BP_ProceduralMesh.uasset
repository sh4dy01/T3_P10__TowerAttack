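; Exercise actor that builds a procedural mesh and lets the player slice it with a plane component.
; The construction script creates the mesh section from variable arrays and applies an unlit texture material instance.
; BeginPlay adds convex collision from that section's vertices and enables player input.
; Pressing F slices at the plane with a new cap section, simulates physics on the slice result, then nudges the plane along its local Z.
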(event `self.ReceiveBeginPlay`
  (bind _proceduralmesh (`self.ProceduralMesh`))
  (bind _vertices (`KismetProceduralMeshLibrary.GetSectionFromProceduralMesh` _proceduralmesh))
  (`ProceduralMeshComponent.AddCollisionConvexMesh` _proceduralmesh _vertices)
  (`self.EnableInput` (`GameplayStatics.GetPlayerController` 0)))

(event `Key|F`
  (params (Key :type "Key Structure"))
  (bind _plane (`self.Plane`))
  (:`Pressed`
    (bind _outotherhalfprocmesh (`KismetProceduralMeshLibrary.SliceProceduralMesh` (`self.ProceduralMesh`) (`SceneComponent.K2_GetComponentLocation` _plane) (`SceneComponent.GetUpVector` _plane) true "CreateNewSectionForCap"))
    (`PrimitiveComponent.SetSimulatePhysics` _outotherhalfprocmesh true)
    (`SceneComponent.K2_AddLocalOffset` (`self.Plane`) (0.0 0.0 10.0) false false)))

(fn `UserConstructionScript`
  (`ProceduralMeshComponent.CreateMeshSection_LinearColor` :`self` (`self.ProceduralMesh`) :`Vertices` (`self.Vertices`) :`Triangles` (`self.Indices`) :`UV0` (`self.UV0`) :`VertexColors` (`self.Vertex Colors`))
  (`PrimitiveComponent.CreateDynamicMaterialInstance` (`self.ProceduralMesh`) 0 "/Game/Game/Art/Materials/Other/Exercises/M_UnlitTexture.M_UnlitTexture" "None"))