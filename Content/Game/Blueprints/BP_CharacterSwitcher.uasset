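; BP_CharacterSwitcher lets the player swap between a roster of playable characters, with one active at a time.
; On BeginPlay it pre-spawns every available class deactivated, and InitializeWithCharacter activates the starting one.
; SwitchCharacter takes a one-based slot, deactivates and unpossesses the current character, then activates the target with the old velocity, transform and camera rotation.
; Each switch broadcasts OnCharacterSwitch and starts a short cooldown.
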(event `self.ReceiveBeginPlay`
  (`|ExecutionSequence`
    (:`then_0`
      (for _array_element (`self.AvailableCharacter`)
        (bind _returnvalue (`|SpawnActorFromClass` _array_element (`self.GetTransform`) "AdjustIfPossibleButAlwaysSpawn" "MultiplyWithRoot" null null))
        (`/Engine/EditorBlueprintResources/StandardMacros.IsValid` _returnvalue
          (:`Is Valid`
            (`/Game/Game/Blueprints/Characters/BP_CharacterBase.Deactivate` _returnvalue)
            (`KismetArrayLibrary.Array_AddUnique` (`self.SpawnedCharacters`) _returnvalue)))))))

(event `StartSwitchCooldown`
  (if (`self.CanSwitch`)
    (set `self.CanSwitch` false)
    (`KismetSystemLibrary.Delay` 0.2)
    (set `self.CanSwitch` true)))

(fn `GetCurrentCharacter`
  (returns (CurrentCharacter :type "/Game/Game/Blueprints/Characters/BP_CharacterBase Object Reference"))
  (return (`self.CurrentCharacter`)))

(fn `InitializeWithCharacter`
  (params (NewParam :type Integer))
  (bind _spawnedcharacters (`self.SpawnedCharacters`))
  (if (`KismetArrayLibrary.Array_IsValidIndex` _spawnedcharacters NewParam)
    (bind _output_get (set `self.CurrentCharacter` (`|GetArrayItem` _spawnedcharacters NewParam)))
    (`/Game/Game/Blueprints/Characters/BP_CharacterBase.Activate` _output_get)
    (`self.OnCharacterSwitch` _output_get)
    (return)))

(fn `SwitchCharacter`
  (params (SelectedCharacter :type Integer))
  (locals (OldVelocity :type "Vector Structure") (DesiredCharacter :type "/Game/Game/Blueprints/Characters/BP_CharacterBase Class Reference") (DesiredIndex :type Integer) (OldTransform :type "Transform Structure") (OldCameraRotation :type "Rotator Structure" :default (struct)))
  (bind _returnvalue (- SelectedCharacter 1))
  (bind _currentcharacter (`self.CurrentCharacter`))
  (bind (_oldtransform_location _oldtransform_rotation) (`KismetMathLibrary.BreakTransform` (`local.OldTransform`)))
  (bind _output (`|GetArrayItem` (`self.AvailableCharacter`) _returnvalue))
  (if (`self.CanSwitch`)
    ;[1 1 1] Verify if the selected class is valid
    (if (`KismetSystemLibrary.IsValidClass` _output)
      (set `local.DesiredCharacter` _output)
      ;[1 1 1] Verify if we are selecting an other character
      (if (!= _returnvalue (`self.CurrentPlayerIndex`))
        ;[1 1 1] Check if the index is valid
        (if (`KismetArrayLibrary.Array_IsValidIndex` (`self.SpawnedCharacters`) _returnvalue)
          (set `local.DesiredIndex` _returnvalue)
          (`|ExecutionSequence`
            (:`then_0`
              ;[1 1 1] Get old character data
              (set `local.OldVelocity` (`MovementComponent.Velocity` (`Character.CharacterMovement` _currentcharacter)))
              (set `local.OldTransform` (`self.GetTransform` _currentcharacter))
              (set `local.OldCameraRotation` (`Pawn.GetControlRotation` _currentcharacter)))
            (:`then_1`
              ;[1 1 1] Deactivate current character
              (`/Game/Game/Blueprints/Characters/BP_CharacterBase.Deactivate` (`self.CurrentCharacter`))
              (`Controller.UnPossess` (`GameplayStatics.GetPlayerController` 0)))
            (:`then_2`
              ;[1 1 1] Select new character
              (set `self.CurrentPlayerIndex` (`local.DesiredIndex`))
              (set `self.CurrentCharacter` (`|GetArrayItem` (`self.SpawnedCharacters`) (`local.DesiredIndex`)))
              (`self.OnCharacterSwitch` (`self.CurrentCharacter`)))
            (:`then_3`
              ;[1 1 1] Set new character data
              (`/Game/Game/Blueprints/Characters/BP_CharacterBase.Initialize` (`self.CurrentCharacter`) (`local.OldVelocity`) _oldtransform_location _oldtransform_rotation)
              (`/Game/Game/Blueprints/Characters/BP_CharacterBase.Activate` (`self.CurrentCharacter`)))
            (:`then_4`
              ;[1 1 1] End of the method
              (`self.StartSwitchCooldown`)
              (`Controller.SetControlRotation` (`GameplayStatics.GetPlayerController` 0) (`local.OldCameraRotation`))
              (return))))))))

(fn `UserConstructionScript`)