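; BP_Enzo is the character Blueprint for Enzo, whose abilities are arrow shooting, scatter, climbing and bullet time.
; On BeginPlay it runs the parent logic, then initializes each ability, passing the capsule to Climb and ShootArrow, plus movement and a line end location to Climb and an arrow to ShootArrow.
; It then registers them with CharacterAttackManager as primary attack, secondary attack and two spells.
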(event `self.ReceiveBeginPlay`
  (`parent.ReceiveBeginPlay`)
  (`/Game/Game/Blueprints/Components/Attacks/Characters/Enzo/BPC_Climb.Init` (`self.Climb`) (`self.LineEndLocation`) (`self.CapsuleComponent`) (`self.CharacterMovement`))
  (`/Game/Game/Blueprints/Components/Attacks/Characters/Enzo/BPC_ShootArrow.Init` (`self.ShootArrow`) (`self.BArrow`) (`self.CapsuleComponent`))
  (`/Game/Game/Blueprints/Components/Attacks/Characters/Enzo/BPC_Scatter.Init` (`self.Scatter`) null null)
  (`/Game/Game/Blueprints/Components/Attacks/Characters/Enzo/BPC_BulletTime.Init` (`self.BulletTime`))
  (`/Game/Game/Blueprints/Components/Attacks/BPC_AttackManager.Initialize` (`self.Character Attack Manager`) (`self.ShootArrow`) (`self.Scatter`) (`self.Climb`) (`self.BulletTime`)))

(fn `UserConstructionScript`
  (`parent.UserConstructionScript`))