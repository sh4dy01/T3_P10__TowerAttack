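; Scotty is a player character with sword attacks, a grab-and-throw spell and a charge spell.
; Primary attack cycles combo montages or plays an in-air montage, locking movement until blend-out; sword overlaps apply damage looked up by combo index.
; A per-tick camera trace highlights tagged BP_GrabbableItems, which the first spell grabs at a socket or launches by impulse.
; Holding the second spell hides the sword, forces forward movement and animates FOV.
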(event `self.Sword.OnComponentBeginOverlap`
  (params (OverlappedComponent :type "PrimitiveComponent Object Reference") (OtherActor :type "Actor Object Reference") (OtherComp :type "PrimitiveComponent Object Reference") (OtherBodyIndex :type Integer) (bFromSweep :type Boolean) (SweepResult :type "HitResult Structure (by ref)"))
  ;[0.4048 0.9602 1] Attack animation
  ;;[1 0.6196 0.5698] Sword Damage
  (`GameplayStatics.ApplyDamage` null (`BlueprintMapLibrary.Map_Find` (`self.Damages`) (`self.CurrentAnimMontage`))))

(event `EnhancedInput|/Game/Game/Inputs/Actions/IA_PrimaryAttack`
  (params (ActionValue :type Boolean) (ElapsedSeconds :type "Float (double-precision)") (TriggeredSeconds :type "Float (double-precision)") (InputAction :type "InputAction Object Reference" :default "/Game/Game/Inputs/Actions/IA_PrimaryAttack.IA_PrimaryAttack"))
  ;[0.4048 0.9602 1] Attack animation
  (:`Started`
    (if (not (`self.IsBusy`))
      (set `CharacterMovementComponent.MaxWalkSpeed` 0.0 (`self.CharacterMovement`))
      (set `self.IsBusy` true)
      (if (`NavMovementComponent.IsFalling` (`self.CharacterMovement`))
        ;;[0.5212 1 0.6338] Play 'in-air' anim montage if the player is falling
        (`|PlayMontage` (`self.Mesh`) (`self.InAirAttackMontage`)
          (:`OnBlendOut`
            (set `self.IsBusy` false)
            (set `CharacterMovementComponent.MaxWalkSpeed` 600.0 (`self.CharacterMovement`))))
        (else
          ;;[0.4646 1 0.5279] Play next animation in combo
          (`|PlayMontage` (`self.Mesh`) (`|GetArrayItem` (`self.AttackAnimMontages`) (`self.CurrentAnimMontage`))
            (:`OnBlendOut`
              (bind _result (`/Engine/EditorBlueprintResources/StandardMacros.IncrementInt` (`self.CurrentAnimMontage`))
                (:`  `
                  (set `self.CurrentAnimMontage` (mod _result (`KismetArrayLibrary.Array_Length` (`self.AttackAnimMontages`))))
                  (set `self.IsBusy` false)
                  (set `CharacterMovementComponent.MaxWalkSpeed` 600.0 (`self.CharacterMovement`)))))))))))

(event `EnhancedInput|/Game/Game/Inputs/Actions/IA_FirstSpell`
  (params (ActionValue :type Boolean) (ElapsedSeconds :type "Float (double-precision)") (TriggeredSeconds :type "Float (double-precision)") (InputAction :type "InputAction Object Reference" :default "/Game/Game/Inputs/Actions/IA_FirstSpell.IA_FirstSpell"))
  (bind _hightlightitem (`self.HightlightItem`))
  ;[0.6614 0.655 1] Grab Operation
  (:`Started`
    (`/Engine/EditorBlueprintResources/StandardMacros.IsValid` (`self.GrabbedObject`)
      (:`Is Valid`
        (`/Game/Game/Blueprints/Items/BP_GrabbableItem.OnLauch` (`self.GrabbedObject`))
        (`PhysicsHandleComponent.ReleaseComponent` (`self.Grabber`))
        (`PrimitiveComponent.AddImpulse` (`/Game/Game/Blueprints/Items/BP_GrabbableItem.Mesh` (`self.GrabbedObject`)) (* (`SceneComponent.GetForwardVector` (`self.Camera`)) (`self.ThrowPower`)) "None" false)
        (set `self.GrabbedObject` null))
      (:`Is Not Valid`
        (`/Engine/EditorBlueprintResources/StandardMacros.IsValid` _hightlightitem
          (:`Is Valid`
            (`PhysicsHandleComponent.GrabComponentAtLocation` (`self.Grabber`) (`/Game/Game/Blueprints/Items/BP_GrabbableItem.Mesh` _hightlightitem) "None" (`self.K2_GetActorLocation` _hightlightitem))
            (set `self.GrabbedObject` (`self.HightlightItem`))))))))

(event `EnhancedInput|/Game/Game/Inputs/Actions/IA_SecondSpell`
  (params (ActionValue :type Boolean) (ElapsedSeconds :type "Float (double-precision)") (TriggeredSeconds :type "Float (double-precision)") (InputAction :type "InputAction Object Reference" :default "/Game/Game/Inputs/Actions/IA_SecondSpell.IA_SecondSpell"))
  (bind _sword (`self.Sword`))
  (bind _sword_2 (`self.Sword`))
  ;[1 0.577 0.9436] Charge attack
  (:`Started`
    (`SceneComponent.SetHiddenInGame` _sword_2 true false)
    (`PrimitiveComponent.SetCollisionEnabled` _sword_2 "NoCollision")
    (set `CharacterMovementComponent.MaxWalkSpeed` (`self.ChargeSpeed`) (`self.CharacterMovement`))
    (`ActorComponent.Activate` (`self.Charge`) false)
    (bind (_direction _fov) (`Timeline|Camera FOV Change` :!via `PlayFromStart` :!label _label)
      (:`Update`
        (`CameraComponent.SetFieldOfView` (`self.Camera`) _fov))))
  (:`Ongoing`
    (`self.AddMovementInput` (`SceneComponent.GetForwardVector` (`self.CapsuleComponent`))))
  (:`Completed`
    (`SceneComponent.SetHiddenInGame` _sword false false)
    (`PrimitiveComponent.SetCollisionEnabled` _sword "QueryOnly")
    (set `CharacterMovementComponent.MaxWalkSpeed` 600.0 (`self.CharacterMovement`))
    (`TimelineComponent.SetPlayRate` (`self.Camera FOV Change`) 2.5)
    (`ActorComponent.Deactivate` (`self.Charge`))
    (goto _label :!via `ReverseFromEnd`)))

(event `self.ReceiveTick`
  (params (DeltaSeconds :type "Float (single-precision)"))
  ;[1 1 1] Tick
  (`self.CheckForGrabbableInSight`)
  ;;[1 1 1] Grabbed Object Update
  (`/Engine/EditorBlueprintResources/StandardMacros.IsValid` (`self.GrabbedObject`)
    (:`Is Valid`
      (`PhysicsHandleComponent.SetTargetLocation` (`self.Grabber`) (`SceneComponent.K2_GetComponentLocation` (`self.GrabSocket`))))))

(fn `CheckForGrabbableInSight`
  (locals (HitResult :type "HitResult Structure") (bHit :type Boolean))
  (bind _hightlightitem (`self.HightlightItem`))
  (bind _camera (`self.Camera`))
  (bind _hightlightitem_2 (`self.HightlightItem`))
  (bind (_bblockinghit _binitialoverlap _time _distance _location _impactpoint _normal _impactnormal _physmat _hitactor) (`GameplayStatics.BreakHitResult` (`local.HitResult`)))
  (bind _returnvalue (`SceneComponent.K2_GetComponentLocation` _camera))
  ;[1 1 1] Check in front of the player
  (bind (_outhit _returnvalue_2) (`KismetSystemLibrary.LineTraceSingle` _returnvalue (+ _returnvalue (* (`SceneComponent.GetForwardVector` _camera) (`self.GrabRange`))) "TraceTypeQuery1" false (`|MakeArray` self :!type "Actor Object Reference") "None" true (struct :`R` 1.0 :`G` 0.354083 :`B` 0.916096 :`A` 1.0) (struct :`G` 1.0 :`A` 1.0) 2.0))
  ;[1 1 1] Did we hit something.
  (bind _output_get (set `local.bHit` _returnvalue_2))
  (if _output_get
    ;[1 1 1] Is the last object in memory ?
    (bind _output_get_2 (set `local.HitResult` _outhit))
    (if (== (`self.HightlightItem`) (`.HitActor` (`GameplayStatics.BreakHitResult` _output_get_2)))
      ;[1 1 1] Still the same object so nothing changed
      (return)
      (else
        ;[1 1 1] We do not hightlight the last object in memory, so we reset it
        (`/Engine/EditorBlueprintResources/StandardMacros.IsValid` _hightlightitem
          (:`Is Valid`
            (`/Game/Game/Blueprints/Items/BP_GrabbableItem.ResetHightlight` _hightlightitem))
          (:`Is Not Valid`
            _))
        ;[1 1 1] Is the new object grabbable ?
        (if (`self.ActorHasTag` _hitactor (`self.GrabTag`))
          ;[1 1 1] Hightlight
          (bind _asbp_grabbable_item (cast `/Game/Game/Blueprints/Items/BP_GrabbableItem` _hitactor))
          (`/Game/Game/Blueprints/Items/BP_GrabbableItem.HightLightObject` _asbp_grabbable_item)
          (set `self.HightlightItem` _asbp_grabbable_item)
          (else
            (set `self.HightlightItem` null)))))
    (else
      (`/Engine/EditorBlueprintResources/StandardMacros.IsValid` _hightlightitem_2
        (:`Is Valid`
          (`/Game/Game/Blueprints/Items/BP_GrabbableItem.ResetHightlight` _hightlightitem_2)
          (set `self.HightlightItem` null))))))

(fn `UserConstructionScript`
  (`parent.UserConstructionScript`))