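; Charge hit trigger for Scotty that breaks and scatters Geometry Collection structures on contact.
; Collision starts disabled and is toggled through Activate and Deactivate.
; Each hit applies radial Field System forces from the explosion zone: external cluster strain to fracture, then culled radial linear velocity to push pieces.
; A DoOnce with a delayed reset throttles the camera shake and hit sound, while the physics fields fire on every hit.
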(event `Init`
  (params (CameraComp :type "CameraComponent Object Reference"))
  (set `self.Camera Comp` CameraComp))

(event `self.ReceiveBeginPlay`
  (`self.Deactivate`))

(event `self.Trigger.OnComponentHit`
  (params (HitComponent :type "PrimitiveComponent Object Reference") (OtherActor :type "Actor Object Reference") (OtherComp :type "PrimitiveComponent Object Reference") (NormalImpulse :type "Vector Structure") (Hit :type "HitResult Structure (by ref)"))
  (bind _onhitexplosionzone (`self.OnHitExplosionZone`))
  (bind _returnvalue (`RadialFalloff.SetRadialFalloff` (`self.RadialFalloff`) (`self.ExplosionMagnitude`) 0.0 1.0 0.0 (`SphereComponent.GetScaledSphereRadius` _onhitexplosionzone) (`SceneComponent.K2_GetComponentLocation` _onhitexplosionzone) "Field_Falloff_Linear"))
  ;[1 1 1] Handle Collision With Any Object
  (cast `GeometryCollectionActor` OtherActor)
  (`FieldSystemComponent.ApplyPhysicsField` (`self.FieldSystemComponent`) true "Field_ExternalClusterStrain" null _returnvalue)
  (`FieldSystemComponent.ApplyPhysicsField` (`self.FieldSystemComponent`) true "Field_LinearVelocity" null (`CullingField.SetCullingField` (`self.CullingField`) _returnvalue (`RadialVector.SetRadialVector` (`self.RadialVector`) (`self.ExplosionVelocityMagnitude`) (`SceneComponent.K2_GetComponentLocation` (`self.OnHitExplosionZone`))) "Field_Culling_Outside"))
  (`/Engine/EditorBlueprintResources/StandardMacros.DoOnce` false :!label _label
    (:`Completed`
      (`GameplayStatics.PlayWorldCameraShake` "/Game/Game/Blueprints/Characters/Scotty/Effects/BP_ScottyCameraShake_ChargeHit.BP_ScottyCameraShake_ChargeHit_C" (`SceneComponent.K2_GetComponentLocation` (`self.Camera Comp`)) 0.0 1000.0)
      (`GameplayStatics.PlaySoundAtLocation` (`self.HitSound`) (`.Location` (`GameplayStatics.BreakHitResult` Hit)) (struct) (`self.HitSoundVolumeMultiplier`) 1.0 0.0 null null null null)
      (`KismetSystemLibrary.Delay` 1.5)
      (goto _label :!via `Reset`))))

(fn `Activate`
  (`PrimitiveComponent.SetCollisionEnabled` (`self.Trigger`) "QueryAndPhysics"))

(fn `Deactivate`
  (`PrimitiveComponent.SetCollisionEnabled` (`self.Trigger`) "NoCollision"))

(fn `UserConstructionScript`)