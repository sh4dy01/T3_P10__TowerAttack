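; BP_Juan is the character Blueprint for Juan, with a primary attack and a shield spell as his first spell.
; On BeginPlay it casts the ShieldScanner child actor to BP_ShieldScanner, hides its mesh and passes it to the ShieldSpell's Init.
; It then registers PrimaryAttack and ShieldSpell with the CharacterAttackManager, which is skipped if the cast fails.
; The construction script only calls the parent's.
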(event `self.ReceiveBeginPlay`
  (bind _asbp_shield_scanner (cast `/Game/Game/Blueprints/Characters/Juan/BP_ShieldScanner` (`ChildActorComponent.ChildActor` (`self.ShieldScanner`))))
  (`SceneComponent.SetVisibility` (`/Game/Game/Blueprints/Characters/Juan/BP_ShieldScanner.Mesh` _asbp_shield_scanner) false false)
  (`/Game/Game/Blueprints/Components/Attacks/Characters/Juan/BPC_ShieldSpell.Init` (`self.Shield Spell`) _asbp_shield_scanner)
  (`/Game/Game/Blueprints/Components/Attacks/BPC_AttackManager.Initialize` (`self.Character Attack Manager`) (`self.Primary Attack`) null (`self.Shield Spell`) null))

(fn `UserConstructionScript`
  (`parent.UserConstructionScript`))