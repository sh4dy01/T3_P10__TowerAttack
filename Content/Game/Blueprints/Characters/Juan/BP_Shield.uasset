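; BP_Shield is a shield actor that dissolves in, drops downward and comes to rest on the world.
; BeginPlay creates a dissolve material instance stamped with real time, then after a short delay enables physics and applies a strong downward impulse.
; Hits against static or dynamic world objects switch physics off and print the hit component's name.
; NukeSelf flips the dissolve to disappearing, then destroys the actor after the same delay.
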(event `self.ReceiveBeginPlay`
  (bind _returnvalue (`PrimitiveComponent.CreateDynamicMaterialInstance` (`self.Shield`) 0 "/Game/Game/Art/Materials/Guillaume/M_Dissolve.M_Dissolve" "None"))
  (bind _output_get (set `self.MaterialRef` _returnvalue))
  (`MaterialInstanceDynamic.SetScalarParameterValue` _output_get "LaunchTimeSeconds" (`GameplayStatics.GetRealTimeSeconds`))
  (`KismetSystemLibrary.Delay` 0.4)
  (`PrimitiveComponent.SetSimulatePhysics` (`self.Shield`) true)
  (`PrimitiveComponent.AddImpulse` (`self.Shield`) (0.0 0.0 -5000.0) "None" true))

(event `self.Shield.OnComponentHit`
  (params (HitComponent :type "PrimitiveComponent Object Reference") (OtherActor :type "Actor Object Reference") (OtherComp :type "PrimitiveComponent Object Reference") (NormalImpulse :type "Vector Structure") (Hit :type "HitResult Structure (by ref)"))
  (bind _returnvalue (`PrimitiveComponent.GetCollisionObjectType` OtherComp))
  (`/Engine/EditorBlueprintResources/StandardMacros.IsValid` OtherComp
    (:`Is Valid`
      (if (or (`|EnumEquality` _returnvalue "ECC_WorldStatic") (`|EnumEquality` _returnvalue "ECC_WorldDynamic"))
        (`PrimitiveComponent.SetSimulatePhysics` (`self.Shield`) false)
        (`KismetSystemLibrary.PrintString` (`KismetSystemLibrary.GetDisplayName` OtherComp))))))

(event `NukeSelf`
  (bind _materialref (`self.MaterialRef`))
  (`MaterialInstanceDynamic.SetScalarParameterValue` _materialref "LaunchTimeSeconds" (`GameplayStatics.GetRealTimeSeconds`))
  (`MaterialInstanceDynamic.SetScalarParameterValue` _materialref "IsAppearing" 0.0)
  (`KismetSystemLibrary.Delay` 0.4)
  (`self.K2_DestroyActor`))

(fn `UserConstructionScript`)