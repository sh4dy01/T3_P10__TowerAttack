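; BP_Platform is a temporary rock platform actor that dissolves in on spawn and dissolves away when its lifetime ends.
; On BeginPlay it creates a dynamic M_Dissolve material on the RockPlatformD mesh, stamps the current real time to drive the effect, then waits for TTL.
; NukeSelf flips IsAppearing to zero, restamps the time to play the fade-out, and destroys the actor shortly after.
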(event `self.ReceiveBeginPlay`
  (bind _returnvalue (`PrimitiveComponent.CreateDynamicMaterialInstance` (`self.Rock_Platform_D`) 0 "/Game/Game/Art/Materials/Guillaume/M_Dissolve.M_Dissolve" "None"))
  (bind _output_get (set `self.MaterialRef` _returnvalue))
  (`MaterialInstanceDynamic.SetScalarParameterValue` _output_get "LaunchTimeSeconds" (`GameplayStatics.GetRealTimeSeconds`))
  (`KismetSystemLibrary.Delay` (`self.TTL`))
  (`self.NukeSelf`))

(event `NukeSelf`
  (`MaterialInstanceDynamic.SetScalarParameterValue` (`self.MaterialRef`) "IsAppearing" 0.0)
  (`MaterialInstanceDynamic.SetScalarParameterValue` (`self.MaterialRef`) "LaunchTimeSeconds" (`GameplayStatics.GetRealTimeSeconds`))
  (`KismetSystemLibrary.Delay` 0.4)
  (`self.K2_DestroyActor`))

(fn `UserConstructionScript`)