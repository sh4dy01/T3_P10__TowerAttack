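; BP_ShieldScanner is a scanner actor in Juan's character folder that detects whether its mesh overlaps anything and shows that as an invalid state.
; The construction script gives the mesh a dynamic M_ShieldScanner material.
; Mesh overlap events count overlaps, toggling the IsOverlapping flag and the material's IsInvalid parameter.
; The state clears only when the last overlap ends.
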(event `self.Mesh.OnComponentBeginOverlap`
  (params (OverlappedComponent :type "PrimitiveComponent Object Reference") (OtherActor :type "Actor Object Reference") (OtherComp :type "PrimitiveComponent Object Reference") (OtherBodyIndex :type Integer) (bFromSweep :type Boolean) (SweepResult :type "HitResult Structure (by ref)"))
  (`/Engine/EditorBlueprintResources/StandardMacros.IncrementInt` (`self.NumberOfOverlap`)
    (:`  `
      (`MaterialInstanceDynamic.SetScalarParameterValue` (`self.MaterialInstanceRef`) "IsInvalid" 1.0)
      (set `self.IsOverlapping` true))))

(event `self.Mesh.OnComponentEndOverlap`
  (params (OverlappedComponent :type "PrimitiveComponent Object Reference") (OtherActor :type "Actor Object Reference") (OtherComp :type "PrimitiveComponent Object Reference") (OtherBodyIndex :type Integer))
  (bind _result (`/Engine/EditorBlueprintResources/StandardMacros.DecrementInt` (`self.NumberOfOverlap`))
    (:`  `
      (if (<= _result 0)
        (set `self.NumberOfOverlap` (`KismetMathLibrary.Clamp` (`self.NumberOfOverlap`)))
        (`MaterialInstanceDynamic.SetScalarParameterValue` (`self.MaterialInstanceRef`) "IsInvalid" 0.0)
        (set `self.IsOverlapping` false)))))

(fn `UserConstructionScript`
  (bind _returnvalue (`PrimitiveComponent.CreateDynamicMaterialInstance` (`self.Mesh`) 0 "/Game/Game/Art/Materials/Guillaume/M_ShieldScanner.M_ShieldScanner" "None"))
  (set `self.MaterialInstanceRef` _returnvalue))