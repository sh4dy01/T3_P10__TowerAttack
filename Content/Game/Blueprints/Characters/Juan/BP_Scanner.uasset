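; BP_Scanner is a placement-check actor in Juan's character folder that shows whether its mesh overlaps something, using the M_ShieldScanner material.
; The construction script creates a dynamic instance of that material on the mesh.
; BeginOverlap and EndOverlap keep an overlap count, setting the IsInvalid parameter and IsOverlapping flag on entry and clearing both only when none remain.
; Both functions have no callers in this Blueprint, and its event graph is empty.
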(fn `BeginOverlap`
  (`/Engine/EditorBlueprintResources/StandardMacros.IncrementInt` (`self.NumberOfOverlap`)
    (:`  `
      (`MaterialInstanceDynamic.SetScalarParameterValue` (`self.MaterialRef`) "IsInvalid" 1.0)
      (set `self.IsOverlapping` true))))

(fn `EndOverlap`
  (bind _result (`/Engine/EditorBlueprintResources/StandardMacros.DecrementInt` (`self.NumberOfOverlap`))
    (:`  `
      (if (<= _result 0)
        (set `self.NumberOfOverlap` (`KismetMathLibrary.Clamp` _result))
        (`MaterialInstanceDynamic.SetScalarParameterValue` (`self.MaterialRef`) "IsInvalid" 0.0)
        (set `self.IsOverlapping` false)))))

(fn `UserConstructionScript`
  (bind _returnvalue (`PrimitiveComponent.CreateDynamicMaterialInstance` (`self.Mesh`) 0 "/Game/Game/Art/Materials/Guillaume/M_ShieldScanner.M_ShieldScanner" "None"))
  (set `self.MaterialRef` _returnvalue))