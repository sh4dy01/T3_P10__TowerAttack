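; Base character Blueprint for switchable player characters, with activate/deactivate toggling tick, collision, visibility and the safe-zone timer.
; Activation plays a switch montage, while deactivation disables input and cancels the current attack.
; A looping timer supports saving grounded positions for respawning, and a health-component death delegate is bound, with OnDeath restarting the level.
; Helpers control sprint, gravity, jump and input; landing restores gravity and shakes the camera.
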(event `self.ReceiveBeginPlay`
  (set `self.BaseWalkSpeed` (`CharacterMovementComponent.MaxWalkSpeed` (`self.CharacterMovement`)))
  (set `self.BaseGravityScale` (`CharacterMovementComponent.GravityScale` (`self.CharacterMovement`)))
  (set `self.SafeZonePosition` (`self.K2_GetActorLocation`))
  (bind _returnvalue (`KismetSystemLibrary.K2_SetTimerDelegate` (`|CreateDelegate` :!event `TrySetSafeZonePos`) 1.0 true))
  (set `self.SafeZoneTimerHandle` _returnvalue)
  (add `/Game/Game/Blueprints/Components/BPC_HealthComponent.OnDeathDelegate` (`self.HealthComponent`) (`|CreateDelegate` :!event `OnDeath`)))

(event `OnActivation`
  (`|PlayMontage` (`self.Mesh`) (`self.SwitchAnim`) 1.5))

(event `OnDeactivation`
  (`/Game/Game/Blueprints/Components/Attacks/BPC_AttackManager.TryCancelCurrentAttack` (`self.Character Attack Manager`)))

(event `self.OnLanded`
  (params (Hit :type "HitResult Structure (by ref)"))
  (bind (_returnvalue_x _returnvalue_y _returnvalue_z) (`KismetMathLibrary.BreakVector` (`CharacterMovementComponent.GetLastUpdateVelocity` (`self.CharacterMovement`))))
  (`self.RevertGravityScale`)
  (`PlayerCameraManager.StartCameraShake` :`self` (`GameplayStatics.GetPlayerCameraManager` 0) :`ShakeClass` "/Game/Game/Blueprints/BP_CameraShakeOnLand.BP_CameraShakeOnLand_C" :`Scale` (+ 1.0 (* (`self.JumpHeld`) (`KismetMathLibrary.FClamp` (/ (`KismetMathLibrary.Abs` _returnvalue_z) 50.0))))))

(fn `Activate`
  (`self.SetActorTickEnabled` true)
  (`KismetSystemLibrary.K2_UnPauseTimerHandle` (`self.SafeZoneTimerHandle`))
  (`self.SetActorEnableCollision` true)
  (`self.SetActorHiddenInGame` false)
  (`self.OnActivation`)
  (return))

(fn `ActivateInput`
  (bind _returnvalue (`GameplayStatics.GetPlayerController` 0))
  (`self.EnableInput` _returnvalue _returnvalue)
  (return))

(fn `ActivateMovement`
  (`Controller.SetIgnoreMoveInput` (`GameplayStatics.GetPlayerController` 0) false)
  (return))

(fn `ActivateSprint`
  (set `CharacterMovementComponent.MaxWalkSpeed` (* (`self.BaseWalkSpeed`) (`self.SprintModifier`)) (`self.CharacterMovement`))
  (set `self.IsSprinting` true)
  (return))

(fn `CancelSprint`
  (set `CharacterMovementComponent.MaxWalkSpeed` (`self.BaseWalkSpeed`) (`self.CharacterMovement`))
  (set `self.IsSprinting` false))

(fn `Deactivate`
  (`self.SetActorTickEnabled` false)
  (`KismetSystemLibrary.K2_PauseTimerHandle` (`self.SafeZoneTimerHandle`))
  (`self.DisableInput` null)
  (`self.SetActorEnableCollision` false)
  (`self.SetActorHiddenInGame` true)
  (`self.OnDeactivation`)
  (return))

(fn `DeactivateInput`
  (bind _returnvalue (`GameplayStatics.GetPlayerController` 0))
  (`self.DisableInput` _returnvalue _returnvalue)
  (return))

(fn `DeactivateMovement`
  (`Controller.SetIgnoreMoveInput` (`GameplayStatics.GetPlayerController` 0) true)
  (return))

(fn `Initialize`
  (params (Velocity :type "Vector Structure") (Position :type "Vector Structure") (Rotation :type "Rotator Structure"))
  (set `MovementComponent.Velocity` Velocity (`self.CharacterMovement`))
  (`self.K2_SetActorLocationAndRotation` Position Rotation false true))

(fn `OnDeath`
  (`KismetSystemLibrary.ExecuteConsoleCommand` "RestartLevel" null))

(fn `RespawnPlayerToSafeZone`
  (`self.K2_SetActorLocation` (`self.SafeZonePosition`) false true)
  ;[1 1 1] Flush input
  (`WidgetBlueprintLibrary.SetInputMode_GameOnly` (`GameplayStatics.GetPlayerController` 0) true)
  (set `MovementComponent.Velocity` (0.0 0.0 0.0) (`self.CharacterMovement`))
  (return))

(fn `RevertGravityScale`
  (set `CharacterMovementComponent.GravityScale` (`self.BaseGravityScale`) (`self.CharacterMovement`))
  (return))

(fn `SetGravityScale`
  (params (GravityScale :type "Float (double-precision)"))
  (set `CharacterMovementComponent.GravityScale` GravityScale (`self.CharacterMovement`))
  (return))

(fn `SetJumpZVelocity`
  (params (Value :type "Float (double-precision)"))
  (set `CharacterMovementComponent.JumpZVelocity` Value (`self.CharacterMovement`))
  (return))

(fn `TrySetSafeZonePos`
  (bind _returnvalue (`NavMovementComponent.IsMovingOnGround` (`self.CharacterMovement`)))
  (bind _returnvalue_2 (not (`NavMovementComponent.IsFalling` (`self.CharacterMovement`))))
  (`KismetSystemLibrary.PrintString` (`KismetStringLibrary.Conv_BoolToString` _returnvalue_2))
  (`KismetSystemLibrary.PrintString` (`KismetStringLibrary.Conv_BoolToString` _returnvalue))
  (if (and _returnvalue_2 _returnvalue)
    (if (!= (`self.SafeZonePosition`) (`self.K2_GetActorLocation`) :`ErrorTolerance` 1.0)
      (`KismetSystemLibrary.PrintString` "Hello")
      (set `self.SafeZonePosition` (`self.K2_GetActorLocation`))
      (return))))

(fn `UserConstructionScript`)