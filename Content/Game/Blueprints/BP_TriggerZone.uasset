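; BP_TriggerZone is a trigger volume that fires OnTriggered when a BP_CharacterBase actor begins overlapping its Box component.
; The IsTriggered flag records that the zone has fired, and IsTriggerOnce decides whether later overlaps fire it again.
; The zone holds no response logic of its own beyond making that call and setting the flag.
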(event `self.Box.OnComponentBeginOverlap`
  (params (OverlappedComponent :type "PrimitiveComponent Object Reference") (OtherActor :type "Actor Object Reference") (OtherComp :type "PrimitiveComponent Object Reference") (OtherBodyIndex :type Integer) (bFromSweep :type Boolean) (SweepResult :type "HitResult Structure (by ref)"))
  (cast `/Game/Game/Blueprints/Characters/BP_CharacterBase` OtherActor)
  (if (or (and (`self.IsTriggered`) (not (`self.IsTriggerOnce`))) (not (`self.IsTriggered`)))
    (`self.OnTriggered`)
    (set `self.IsTriggered` true)))

(fn `UserConstructionScript`)