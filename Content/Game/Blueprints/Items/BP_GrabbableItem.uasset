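; BP_GrabbableItem is a grabbable item actor that can show and clear a color highlight.
; On BeginPlay it creates a dynamic material instance from the mesh's first material slot and applies the reset color.
; HightLightObject and ResetHightlight switch that material's Color parameter between highlight and reset colors, and GetMesh exposes the mesh to other Blueprints.
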(event `self.ReceiveBeginPlay`
  (bind _mesh (`self.Mesh`))
  (bind _returnvalue (`PrimitiveComponent.CreateDynamicMaterialInstance` _mesh 0 (`PrimitiveComponent.GetMaterial` _mesh 0) "None"))
  (set `self.Material` _returnvalue)
  (`self.ResetHightlight`))

(fn `GetMesh`
  (returns (`Primitive Component` :type "PrimitiveComponent Object Reference"))
  (return (`self.Mesh`)))

(fn `HightLightObject`
  (`MaterialInstanceDynamic.SetVectorParameterValue` (`self.Material`) "Color" (`self.HightLightColor`)))

(fn `ResetHightlight`
  (`MaterialInstanceDynamic.SetVectorParameterValue` (`self.Material`) "Color" (`self.HightLightResetColor`)))

(fn `UserConstructionScript`)