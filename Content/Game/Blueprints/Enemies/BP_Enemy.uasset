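; Enemy character base with melee and ranged attacks, health and a dissolve death.
; Attack events set the target it yaws toward and play montages; shooting spawns a homing projectile from the wand socket, while sword overlaps damage player characters.
; Damage feeds the health component of a child-actor health bar, whose death delegate disables collision and controller.
; Tick then drives the dissolve alpha on material and particles before destroying the actor.
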(event `self.ReceiveBeginPlay`
  (bind _asbp_health_bar (cast `/Game/Game/Blueprints/BP_HealthBar` (`ChildActorComponent.ChildActor` (`self.BP_HealthBar`))))
  (`/Game/Game/Blueprints/BP_HealthBar.Init` _asbp_health_bar (`self.MaxHealth`))
  (bind _output_get (set `self.Health Component` (`/Game/Game/Blueprints/BP_HealthBar.HealthComponent` _asbp_health_bar)))
  (add `/Game/Game/Blueprints/Components/BPC_HealthComponent.OnDeathDelegate` _output_get (`|CreateDelegate` :!event `OnDeath`)))

(event `OnDeath`
  (`self.DetachFromControllerPendingDestroy`)
  (`PrimitiveComponent.SetCollisionEnabled` (`self.CapsuleComponent`) "NoCollision")
  (`PrimitiveComponent.SetCollisionEnabled` (`self.Mesh`) "NoCollision")
  (set `self.Target` null)
  (set `self.IsDead` true)
  (`PrimitiveComponent.CreateDynamicMaterialInstance` (`self.Mesh`) 0 (`self.DisolveMaterial`) "None"))

(event `self.ReceiveTick`
  (params (DeltaSeconds :type "Float (single-precision)"))
  (bind _target (`self.Target`)
    (:`then`
      (`self.RotateTowardsTarget` _target))
    (:`else`
      (if (`self.IsDead`)
        (bind _output_get (set `self.CurDeathAlpha` (+ (`self.CurDeathAlpha`) (/ DeltaSeconds (`self.DisolveTime`)))))
        (`MeshComponent.SetScalarParameterValueOnMaterials` (`self.Mesh`) (`self.AlphaParameterName`) _output_get)
        (`FXSystemComponent.SetFloatParameter` (`self.DeathParticles`) (`self.AlphaParameterName`) _output_get)
        (if (>= (`self.CurDeathAlpha`) 1.0)
          (`self.K2_DestroyActor`))))))

(event `OnAttackReceiveExecute`
  (params (Target :type "/Game/Game/Blueprints/Characters/BP_CharacterBase Object Reference"))
  (set `self.Target` Target)
  (`|PlayMontage` (`self.Mesh`) (`self.MeleeMontage`) 0.7
    (:`OnNotifyBegin`
      (set `self.HasHitPlayer` false))))

(event `OnShootReceiveExecute`
  (params (Target :type "/Game/Game/Blueprints/Characters/BP_CharacterBase Object Reference"))
  (bind _returnvalue (`SceneComponent.GetSocketLocation` (`self.Wand`) "ShootSocket"))
  (set `self.Target` Target)
  (`|PlayMontage` (`self.Mesh`) (`self.ShootMontage`)
    (:`then`
      (`KismetSystemLibrary.PrintString` (`KismetStringLibrary.Conv_VectorToString` _returnvalue))
      (bind _returnvalue_2 (`|SpawnActorFromClass` "/Game/Game/Blueprints/Enemies/BP_EnemyProj.BP_EnemyProj_C" (`KismetMathLibrary.MakeTransform` _returnvalue (`KismetMathLibrary.MakeRotFromX` (`KismetMathLibrary.Normal` (- (`self.K2_GetActorLocation` Target) _returnvalue)))) "Undefined" "MultiplyWithRoot" null null))
      (set `ProjectileMovementComponent.HomingTargetComponent` (`/Game/Game/Blueprints/Characters/BP_CharacterBase.Scene` Target) (`/Game/Game/Blueprints/Actors/Projectiles/BP_Projectile.ProjectileMovement` _returnvalue_2)))))

(event `self.ReceiveAnyDamage`
  (params (Damage :type "Float (single-precision)") (DamageType :type "DamageType Object Reference") (InstigatedBy :type "Controller Object Reference") (DamageCauser :type "Actor Object Reference"))
  (bind _health_component (`self.Health Component`))
  (`/Engine/EditorBlueprintResources/StandardMacros.IsValid` _health_component
    (:`Is Valid`
      (`/Game/Game/Blueprints/Components/BPC_HealthComponent.ApplyDamage` _health_component Damage)
      (`|PlayMontage` (`self.Mesh`) (`self.HitMontage`)))))

(event `self.Sword.OnComponentBeginOverlap`
  (params (OverlappedComponent :type "PrimitiveComponent Object Reference") (OtherActor :type "Actor Object Reference") (OtherComp :type "PrimitiveComponent Object Reference") (OtherBodyIndex :type Integer) (bFromSweep :type Boolean) (SweepResult :type "HitResult Structure (by ref)"))
  (bind _asbp_character_base (cast `/Game/Game/Blueprints/Characters/BP_CharacterBase` OtherActor))
  (`GameplayStatics.ApplyDamage` _asbp_character_base (`self.Base Damage`) null self)
  (set `self.HasHitPlayer` true)
  (`NiagaraFunctionLibrary.SpawnSystemAtLocation` "/Game/Game/Art/Particles/NS_Hit.NS_Hit" (`SceneComponent.K2_GetComponentLocation` (`self.HitLocation`))))

(fn `RotateTowardsTarget`
  (params (Other :type "Actor Object Reference"))
  (bind (_returnvalue_roll _returnvalue_pitch _returnvalue_yaw) (`KismetMathLibrary.BreakRotator` (`KismetMathLibrary.FindLookAtRotation` (`self.K2_GetActorLocation`) (`self.K2_GetActorLocation` Other))))
  (`self.K2_SetActorRotation` (`KismetMathLibrary.MakeRotator` 0.0 0.0 _returnvalue_yaw)))

(fn `UserConstructionScript`)