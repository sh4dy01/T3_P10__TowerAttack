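; BP_AnchorChaos is a Chaos anchor field actor that sets the dynamic state of physics bodies within a box volume.
; The construction script registers a dynamic state field command on the FieldSystemComponent.
; A uniform integer from FieldState is culled outside a no-falloff box that follows the Anchor component's world transform.
; The event graph holds only disabled stub events, so nothing runs there.
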(fn `UserConstructionScript`
  (`FieldSystemComponent.AddFieldCommand` (`self.FieldSystemComponent`) true "Field_DynamicState" null (`CullingField.SetCullingField` (`self.CullingField`) (`BoxFalloff.SetBoxFalloff` (`self.BoxFalloff`) 1.0 0.0 1.0 0.0 (`SceneComponent.K2_GetComponentToWorld` (`self.Anchor`)) "Field_FallOff_None") (`UniformInteger.SetUniformInteger` (`self.UniformInteger`) (`KismetMathLibrary.Conv_ByteToInt` (`self.FieldState`))) "Field_Culling_Outside")))