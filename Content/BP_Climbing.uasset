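; BP_Climbing is an unfinished climbing check that detects climbable surfaces for the Enzo actor.
; Each tick it runs a debug-drawn Visibility line trace from Enzo to the LineEndLocation component and checks the hit actor for the Climbable tag.
; On a match it stores how long Space Bar has been held in ClimbTime, otherwise resets it.
; The hold-time threshold branch performs no action, so no climbing movement happens here.
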(event `self.ReceiveTick`
  (params (DeltaSeconds :type "Float (single-precision)"))
  (bind _outhit (`KismetSystemLibrary.LineTraceSingle` :`Start` (`Actor.K2_GetActorLocation` (`self.Enzo`)) :`End` (`SceneComponent.K2_GetComponentLocation` (`self.LineEndLocation`)) :`TraceChannel` "TraceTypeQuery1" :`DrawDebugType` "ForDuration"))
  (if (`Actor.ActorHasTag` (`.HitActor` (`GameplayStatics.BreakHitResult` _outhit)) "Climbable")
    (bind _output_get (set `self.ClimbTime` (`PlayerController.GetInputKeyTimeDown` (`GameplayStatics.GetPlayerController` 0) "SpaceBar")))
    (if (!= _output_get 0.0)
      (if (<= _output_get 0.8)
        _))
    (else
      (set `self.ClimbTime` 0.0))))